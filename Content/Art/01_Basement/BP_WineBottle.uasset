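; BP_WineBottle is a wine bottle prop that feeds its own motion into a liquid material.
; Construction creates a dynamic material instance with a random fill level and seeds the tracked point, offset from the bottle in its rotated frame.
; Each tick derives that point's velocity, smooths the absolute velocity change at a speed-dependent rate, clamps and normalizes it, then writes it to the BottleAcceleration parameter.
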(event `self.ReceiveTick`
  (params (DeltaSeconds :type "Float (single-precision)"))
  (bind (_maxacceleration_x _maxacceleration_y) (`KismetMathLibrary.BreakVector2D` (`self.MaxAcceleration`)))
  (bind _bottle (`self.Bottle`))
  (bind (_maxacceleration_x_2 _maxacceleration_y_2) (`KismetMathLibrary.BreakVector2D` (`self.MaxAcceleration`)))
  (set `self.CurrentPosition` (+ (`SceneComponent.K2_GetComponentLocation` _bottle) (`KismetMathLibrary.GreaterGreater_VectorRotator` (`KismetMathLibrary.Conv_DoubleToVector` (`self.posOffset`)) (`SceneComponent.K2_GetComponentRotation` _bottle))))
  (set `self.Velocity` (/ (- (`self.CurrentPosition`) (`self.LastPosition`)) (`GameplayStatics.GetWorldDeltaSeconds`)))
  (set `self.Acceleration` (`KismetMathLibrary.ClampVectorSize` (`KismetMathLibrary.VInterpTo` (`self.Acceleration`) (`KismetMathLibrary.Vector_GetAbs` (- (`self.Velocity`) (`self.LastVelocity`))) (`GameplayStatics.GetWorldDeltaSeconds`) (`KismetMathLibrary.SelectFloat` 20.0 0.5 (> (`KismetMathLibrary.VSize` (`self.Velocity`)) 25.0))) _maxacceleration_x_2 _maxacceleration_y_2))
  (`MaterialInstanceDynamic.SetVectorParameterValue` (`self.BottleDynamicMat`) "BottleAcceleration" (`KismetMathLibrary.Conv_VectorToLinearColor` (/ (`self.Acceleration`) _maxacceleration_y)))
  (set `self.LastVelocity` (`self.Velocity`))
  (set `self.LastPosition` (`self.CurrentPosition`)))

(fn `UserConstructionScript`
  (bind _posoffset (`self.posOffset`))
  (bind _bottle (`self.Bottle`))
  (bind _returnvalue (+ (`SceneComponent.K2_GetComponentLocation` _bottle) (`KismetMathLibrary.GreaterGreater_VectorRotator` (`KismetMathLibrary.MakeVector` _posoffset _posoffset _posoffset) (`SceneComponent.K2_GetComponentRotation` _bottle))))
  (set `self.LastPosition` _returnvalue)
  (set `self.CurrentPosition` _returnvalue)
  (bind _returnvalue_2 (`PrimitiveComponent.CreateDynamicMaterialInstance` (`self.Bottle`) 0 (`self.BottleMaterial`) "None"))
  (bind _output_get (set `self.BottleDynamicMat` _returnvalue_2))
  (`MaterialInstanceDynamic.SetScalarParameterValue` _output_get "LiquidLevel" (`KismetMathLibrary.RandomFloatInRange` 0.55 0.75)))