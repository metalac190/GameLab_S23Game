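; BP_roots is an art Blueprint that builds tapering spline-mesh geometry, presumably roots, along a spline.
; The construction script adds one Z-forward spline mesh per segment and matches its positions and tangents to the neighboring spline points.
; A running Scale value drops by one over the point count each segment, so each end scale becomes the next start scale for a continuous taper.
; The event graph has no active logic.
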(fn `UserConstructionScript`
  (bind _spline (`self.Spline`))
  (bind _scale (`self.Scale`))
  (bind _scale_2 (`self.Scale`))
  (for _index (range (+ (- (`SplineComponent.GetNumberOfSplinePoints` (`self.Spline`)) 2) 1))
    (bind _returnvalue (`AddComponent|NODE_AddSplineMeshComponent-0`))
    (set `self.Spline Mesh Component` _returnvalue)
    (`SplineMeshComponent.SetForwardAxis` (`self.Spline Mesh Component`) "Z" true)
    (`SceneComponent.K2_AttachToComponent` (`self.Spline Mesh Component`) (`self.DefaultSceneRoot`) "None" "KeepRelative" "KeepRelative" "KeepRelative" true)
    (bind _returnvalue_2 (+ _index 1))
    (`SplineMeshComponent.SetStartAndEnd` (`self.Spline Mesh Component`) (`SplineComponent.GetLocationAtSplinePoint` _spline _index "Local") (`SplineComponent.GetTangentAtSplinePoint` _spline _index "Local") (`SplineComponent.GetLocationAtSplinePoint` _spline _returnvalue_2 "Local") (`SplineComponent.GetTangentAtSplinePoint` _spline _returnvalue_2 "Local") true)
    (`SplineMeshComponent.SetStartScale` (`self.Spline Mesh Component`) (`KismetMathLibrary.MakeVector2D` _scale_2 _scale_2) true)
    (set `self.Scale` (- (`self.Scale`) (/ 1 (`KismetMathLibrary.Conv_IntToDouble` (`SplineComponent.GetNumberOfSplinePoints` (`self.Spline`))))))
    (`SplineMeshComponent.SetEndScale` (`self.Spline Mesh Component`) (`KismetMathLibrary.MakeVector2D` _scale _scale) true)))