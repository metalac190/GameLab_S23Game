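; SqueezePause is a trigger volume that briefly slows the player's squeeze movement, likely as a pause moment within a squeeze passage.
; When PausePlayer is set, a player overlap swaps the player's SqueezeSpeed for SqueezeSpeedDivisor, where higher means slower, then restores the cached original after PauseDuration.
; A PauseStart flag guards re-entry, and a DoOnce that is never reset limits the effect to once per instance.
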(event `self.CollisionComponent.OnComponentBeginOverlap`
  (params (OverlappedComponent :type "PrimitiveComponent Object Reference") (OtherActor :type "Actor Object Reference") (OtherComp :type "PrimitiveComponent Object Reference") (OtherBodyIndex :type Integer) (bFromSweep :type Boolean) (SweepResult :type "HitResult Structure (by ref)"))
  (bind _player (`self.Player`))
  (bind _asbp_player (cast `/Game/Entities/Player/BP_Player` OtherActor))
  (set `self.Player` _asbp_player)
  (if (`self.PausePlayer`)
    (if (not (`self.PauseStart`))
      (set `self.PauseStart` true)
      (`/Engine/EditorBlueprintResources/StandardMacros.DoOnce` false
        (:`Completed`
          (set `self.OriginalSqueezeSpeed` (`/Game/Entities/Player/BP_Player.Squeeze Speed` _player))
          (set `/Game/Entities/Player/BP_Player.Squeeze Speed` (`self.SqueezeSpeedDivisor`) _player) ; The higher this is, the slower youll move
          (`KismetSystemLibrary.Delay` (`self.PauseDuration`))
          (set `/Game/Entities/Player/BP_Player.Squeeze Speed` (`self.OriginalSqueezeSpeed`) (`self.Player`))
          (`KismetSystemLibrary.Delay` 0.2)
          (set `self.PauseStart` false))))))

(fn `UserConstructionScript`)