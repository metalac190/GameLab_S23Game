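; BP_ForceField is a Chaos field actor for breakable objects that applies breaking forces around a sphere component.
; ApplyForce sends an external cluster strain field with no falloff, sized to the sphere's scaled radius and driven by the FieldMagnitude variable.
; It then applies a fixed-strength radial angular velocity field from the sphere's center and prints a debug message.
; Nothing in this file calls ApplyForce.
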(fn `Apply Force`
  (bind _fieldsystemcomponent (`self.FieldSystemComponent`))
  (bind _sphere (`self.Sphere`))
  (bind _returnvalue (`SceneComponent.K2_GetComponentLocation` _sphere))
  (`FieldSystemComponent.ApplyPhysicsField` _fieldsystemcomponent true "Field_ExternalClusterStrain" null (`RadialFalloff.SetRadialFalloff` (`self.RadialFalloff`) (`self.FieldMagnitude`) 0.0 1.0 1.0 (`SphereComponent.GetScaledSphereRadius` _sphere) _returnvalue "Field_FallOff_None"))
  (`FieldSystemComponent.ApplyPhysicsField` _fieldsystemcomponent true "Field_AngularVelociy" null (`RadialVector.SetRadialVector` (`self.RadialVector`) 15.0 _returnvalue))
  (`KismetSystemLibrary.PrintString` "External Strain Added"))

(fn `UserConstructionScript`)