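; BP_TestBranch2 is a breakable branch that cracks apart when the player overlaps its trigger box.
; It skips players whose capsule half-height is exactly 45, likely a crouch check, and otherwise fires once.
; The break calls ApplyForce on a child force field actor and plays a branch sound at the root.
; The construction script registers a child anchor field as an initialization field on the Geometry Collection.
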(event `self.Box.OnComponentBeginOverlap`
  (params (OverlappedComponent :type "PrimitiveComponent Object Reference") (OtherActor :type "Actor Object Reference") (OtherComp :type "PrimitiveComponent Object Reference") (OtherBodyIndex :type Integer) (bFromSweep :type Boolean) (SweepResult :type "HitResult Structure (by ref)"))
  (bind _asbp_player (cast `/Game/Entities/Player/Blueprints/BP_Player` OtherActor))
  (if (not (== (`CapsuleComponent.GetScaledCapsuleHalfHeight` (`Character.CapsuleComponent` _asbp_player)) 45.0))
    (`/Engine/EditorBlueprintResources/StandardMacros.DoOnce` false
      (:`Completed`
        (bind _asbp_force_field (cast `/Game/Systems/BreakableObjects/BP_ForceField` (`ChildActorComponent.ChildActor` (`self.BP_ForceField`))))
        (`/Game/Systems/BreakableObjects/BP_ForceField.Apply Force` _asbp_force_field)
        (`GameplayStatics.PlaySoundAtLocation` "/Game/Systems/BreakableObjects/branch.branch" (`SceneComponent.K2_GetComponentLocation` (`self.DefaultSceneRoot`)) (struct) 1.0 1.0 0.0 null null null null)))))

(fn `UserConstructionScript`
  (bind _asbp_anchor_field (cast `/Game/Systems/BreakableObjects/BP_AnchorField` (`ChildActorComponent.ChildActor` (`self.BP_AnchorField`))))
  (`KismetArrayLibrary.Array_Add` (`GeometryCollectionComponent.InitializationFields` (`self.TestBranch2_GeometryCollection1`)) _asbp_anchor_field))