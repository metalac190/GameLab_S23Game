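; Player equipped item with a liquid mesh whose three-band gradient material is created dynamically in the construction script.
; BeginPlay binds to the player's crafter component, but the item-added handler is empty.
; PourLiquid, triggered by debug key B, only prints "Hello" for one crafter input.
; The bottle-based recolor and timeline-driven fill-height logic is disconnected, as is the color-blend math in CalcNewFluidColor.
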(event Custom|PourLiquid
  (params (LiquidColor1 :type Linear%20Color%20Structure) (WineBottle1 :type BP%20Wine%20Bottle%20Source%20Object%20Reference))
  (switch int (Utilities|Array|Length (Variables|/Game/Systems/Mechanics/Crafting/BPC_Crafter.BPC_Crafter_C|GetInput%20Items (Variables|Default|GetBPC%20Crafter)))
    (:1
      (Development|PrintString "Hello"))))

(event Custom|OnItemAdded
  (params (ItemAdded :type S%20Item%20Data%20Structure)))

(event EventBeginPlay
  (Input|EnableInput (Game|GetPlayerController 0))
  (bind _asbp_player (Utilities|Casting|CastToBP_Player (Game|Player|GetPlayerPawn 0)))
  (bind _output_get (Variables|Default|SetBPC%20Crafter (Variables|/Game/Entities/Player/BP_Player.BP_Player_C|GetBPC_Crafter _asbp_player)))
  (EventDispatchers|BindEventtoItemAdded _output_get (delegate Custom|OnItemAdded)))

(event Input|KeyboardEvents|DebugKeyB
  (params (Key :type Key%20Structure :default "None") (ActionValue :type Input%20Action%20Value%20Structure))
  (:Pressed
    (CallFunction|PourLiquid "(R=0.000000,G=0.000000,B=1.000000,A=1.000000)")))

(fn ConstructionScript
  (bind _returnvalue (Rendering|Material|CreateDynamicMaterialInstance (Variables|Default|GetLiquidMesh) 0 (Variables|Default|GetLiquidMaterial) "DynamicLiquidMaterial" :!class /Script/Engine.PrimitiveComponent))
  (bind _output_get (Variables|Default|SetDynamicLiquidMaterial _returnvalue))
  (Utilities|FlowControl|Sequence
    (:then_0
      (Rendering|Material|SetVectorParameterValue _output_get "Water Gradient - Top" (Math|Color|MakeColor 1.0 1.0 1.0) :!class /Script/Engine.MaterialInstanceDynamic))
    (:then_1
      (Rendering|Material|SetVectorParameterValue _output_get "Water Gradient - Middle" (Math|Color|MakeColor 0.5 0.5 0.5) :!class /Script/Engine.MaterialInstanceDynamic))
    (:then_2
      (Rendering|Material|SetVectorParameterValue _output_get "Water Gradient - Bottom" (Math|Color|MakeColor 0.0 0.0 0.0) :!class /Script/Engine.MaterialInstanceDynamic)
      (Rendering|Material|SetMaterial (Variables|Default|GetLiquidMesh) 0 (Variables|Default|GetDynamicLiquidMaterial))
      (Transformation|SetRelativeScale3D (Variables|Default|GetLiquidMesh) (Variables|Default|GetLiquidScale)))))

(fn MakeNewFluidColor
  (params (FluidColor1 :type Linear%20Color%20Structure) (FluidColor2 :type Linear%20Color%20Structure) (Shade :type Float%20%28double-precision%29))
  (return (Utilities|CalcNewFluidColor FluidColor1 FluidColor2 Shade)))

(fn SetNewFluidColor
  (params (DynLiqMat :type Material%20Instance%20Dynamic%20Object%20Reference) (Parameter :type Name) (NewFluidColor :type Linear%20Color%20Structure))
  (Rendering|Material|SetVectorParameterValue DynLiqMat Parameter NewFluidColor :!class /Script/Engine.MaterialInstanceDynamic)
  (Rendering|Material|SetMaterial (Variables|Default|GetLiquidMesh) 0 (Variables|Default|GetDynamicLiquidMaterial)))

(fn DebugColorMaker
  (params (Color1 :type Linear%20Color%20Structure) (Color2 :type Linear%20Color%20Structure))
  (bind _newfluidcolor (CallFunction|MakeNewFluidColor Color1 Color2 0.0))
  (return (Utilities|String|Append (Utilities|String|ToString(Integer) Color1) " and " (Utilities|String|ToString(Integer) Color2) " makes " (Utilities|String|ToString(Integer) _newfluidcolor))))

(fn SetColorGradients
  (params (Top :type Linear%20Color%20Structure) (Middle :type Linear%20Color%20Structure) (Bottom :type Linear%20Color%20Structure))
  (Utilities|FlowControl|Sequence
    (:then_0
      (CallFunction|SetNewFluidColor (Variables|Default|GetDynamicLiquidMaterial) "Water Gradient - Top" Top))
    (:then_1
      (CallFunction|SetNewFluidColor (Variables|Default|GetDynamicLiquidMaterial) "Water Gradient - Middle" Middle))
    (:then_2
      (CallFunction|SetNewFluidColor (Variables|Default|GetDynamicLiquidMaterial) "Water Gradient - Bottom" Bottom))))