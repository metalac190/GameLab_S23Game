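; BP_WineLiquid is the visual wine-crafting liquid, driven by item-added and item-crafted events from the player's BPCCrafter.
; Added items raise the mesh through timeline scaling up to a cap, emptying it if the crafter's inputs are empty afterwards.
; A dynamic material's three-band gradient lerps from WineColorMap colors, turning green for "acid" crafts and black when emptying.
; CalcNewFluidColor's averaging logic is unconnected, so color mixing is unfinished.
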(event `OnItemAdded`
  (params (ItemAdded :type "/Game/Entities/Gameplay/Items/S_ItemData Structure"))
  (`self.PourLiquid` ItemAdded))

(event `self.ReceiveBeginPlay`
  (bind _asbp_player (cast `/Game/Entities/Player/BP_Player` (`GameplayStatics.GetPlayerPawn` 0)))
  (bind _output_get (set `self.BPC Crafter` (`/Game/Entities/Player/BP_Player.BPC_Crafter` _asbp_player)))
  (`|ExecutionSequence`
    (:`then_0`
      (add `/Game/Systems/Mechanics/Crafting/BPC_Crafter.ItemAdded` _output_get (delegate `OnItemAdded`)))
    (:`then_1`
      (add `/Game/Systems/Mechanics/Crafting/BPC_Crafter.ItemCrafted` _output_get (delegate `OnItemCrafted`)))))

(event `OnItemCrafted`
  (params (ItemCrafted :type "/Game/Entities/Gameplay/Items/S_ItemData Structure"))
  (if (`KismetStringLibrary.Contains` ItemCrafted_ItemName_18_CD23B635439CECA1569C62A2D3CDE386 "acid")
    (bind (_direction _stupidfuckingfloatalpha) (`Timeline|StupidFuckingTimeline` :!via `PlayFromStart`)
      (:`Update`
        (set `self.Liquid Float Alpha` _stupidfuckingfloatalpha)
        (`self.SetColorGradients` (struct :`G` 1.0 :`A` 1.0) (`self.FluidColor`) (`self.Liquid Float Alpha`))))))

(event `EmptyBucket`
  ;[1 0 0 0.5] Bad Wine Craft
  (set `self.EndLiquidScale` (0.3 0.3 0.0))
  (set `self.bCanAddWine` false)
  (bind (_direction _liquidfloatalpha _coloralpha) (`Timeline|LiquidEmpty` :!via `ReverseFromEnd`)
    (:`Update`
      (bind _returnvalue (`KismetMathLibrary.VLerp` (`self.EndLiquidScale`) (`self.StartLiquidScale`) _liquidfloatalpha))
      (`SceneComponent.SetRelativeScale3D` (`self.LiquidMesh`) _returnvalue)
      (`self.SetColorGradients` (struct) (`self.FluidColor`) _coloralpha))
    (:`Finished`
      (set `self.StartLiquidScale` _returnvalue)
      (set `self.bCanAddWine` true))))

(event `PourLiquid`
  (params (item :type "/Game/Entities/Gameplay/Items/S_ItemData Structure"))
  (bind _itemadded_itemname (break `/Game/Entities/Gameplay/Items/S_ItemData` (`self.ItemAdded`)))
  (bind (_startliquidscale_x _startliquidscale_y _startliquidscale_z) (`KismetMathLibrary.BreakVector` (`self.StartLiquidScale`)))
  (bind _itemadded_itemname_2 (break `/Game/Entities/Gameplay/Items/S_ItemData` (`self.ItemAdded`)))
  (bind (_value _returnvalue) (`BlueprintMapLibrary.Map_Find` (`self.WineColorMap`) _itemadded_itemname_2))
  (set `self.FluidColor` (`KismetMathLibrary.SelectColor` _value (struct :`A` 1.0) _returnvalue))
  ;[0 1 0 0.5] Good Wine Craft
  (set `self.ItemAdded` item)
  (if (< _startliquidscale_z 0.2)
    (set `self.EndLiquidScale` (+ (`self.StartLiquidScale`) (0.0 0.0 0.1)))
    (set `self.bCanAddWine` false)
    (bind (_direction _liquidfloatalpha) (`Timeline|LiquidPour` :!via `PlayFromStart`)
      (:`Update`
        (set `self.Liquid Float Alpha` _liquidfloatalpha)
        (bind _returnvalue_2 (`KismetMathLibrary.VLerp` (`self.StartLiquidScale`) (`self.EndLiquidScale`) _liquidfloatalpha))
        (`SceneComponent.SetRelativeScale3D` (`self.LiquidMesh`) _returnvalue_2)
        (`self.SwitchStringColor` _itemadded_itemname))
      (:`Finished`
        (set `self.StartLiquidScale` _returnvalue_2)
        (set `self.bCanAddWine` true)
        (if (`KismetArrayLibrary.Array_IsEmpty` (`/Game/Systems/Mechanics/Crafting/BPC_Crafter.Input Items` (`self.BPC Crafter`)))
          (`self.EmptyBucket`))))
    (else
      (set `self.StartLiquidScale` (0.3 0.3 0.2)))))

(fn `DebugColorMaker`
  (params (Color1 :type "LinearColor Structure") (Color2 :type "LinearColor Structure"))
  (returns (Output :type String))
  (bind _newfluidcolor (`self.MakeNewFluidColor` Color1 Color2))
  (return (`KismetStringLibrary.Concat_StrStr` (`KismetStringLibrary.Conv_ColorToString` Color1) " and " (`KismetStringLibrary.Conv_ColorToString` Color2) " makes " (`KismetStringLibrary.Conv_ColorToString` _newfluidcolor))))

(fn `MakeNewFluidColor`
  (params (FluidColor1 :type "LinearColor Structure") (FluidColor2 :type "LinearColor Structure"))
  (returns (NewFluidColor :type "LinearColor Structure") (OldFluidColor1 :type "LinearColor Structure") (OldFluidColor2 :type "LinearColor Structure"))
  (return (`self.CalcNewFluidColor` FluidColor1 FluidColor2) FluidColor1 FluidColor2))

(fn `Set New Fluid Color`
  (params (DynLiqMat :type "MaterialInstanceDynamic Object Reference") (Parameter :type Name) (NewFluidColor :type "LinearColor Structure"))
  (`MaterialInstanceDynamic.SetVectorParameterValue` DynLiqMat Parameter NewFluidColor)
  (`PrimitiveComponent.SetMaterial` (`self.LiquidMesh`) 0 (`self.DynamicLiquidMaterial`)))

(fn `SetColorGradients`
  (params (ColorToLerpTo :type "LinearColor Structure") (Color :type "LinearColor Structure") (WineLerpAlpha :type "Float (double-precision)"))
  (returns (OutColor :type "LinearColor Structure"))
  (bind _returnvalue (`KismetMathLibrary.LinearColorLerp` Color ColorToLerpTo WineLerpAlpha))
  (`|ExecutionSequence`
    (:`then_0`
      (`self.Set New Fluid Color` (`self.DynamicLiquidMaterial`) "Water Gradient - Top" (* _returnvalue 0.2)))
    (:`then_1`
      (`self.Set New Fluid Color` (`self.DynamicLiquidMaterial`) "Water Gradient - Middle" (* _returnvalue 0.5)))
    (:`then_2`
      (`self.Set New Fluid Color` (`self.DynamicLiquidMaterial`) "Water Gradient - Bottom" (* _returnvalue 0.8))
      (return _returnvalue))))

(fn `UserConstructionScript`
  (bind _returnvalue (`PrimitiveComponent.CreateDynamicMaterialInstance` (`self.LiquidMesh`) 0 (`self.LiquidMaterial`) "DynamicLiquidMaterial"))
  (bind _output_get (set `self.DynamicLiquidMaterial` _returnvalue))
  (`|ExecutionSequence`
    (:`then_0`
      (`MaterialInstanceDynamic.SetVectorParameterValue` _output_get "Water Gradient - Top" (`KismetMathLibrary.HSVToRGB` 100.0 1.0 50.0 0.5)))
    (:`then_1`
      (`MaterialInstanceDynamic.SetVectorParameterValue` _output_get "Water Gradient - Middle" (`KismetMathLibrary.HSVToRGB` 100.0 1.0 50.0 0.5)))
    (:`then_2`
      (`MaterialInstanceDynamic.SetVectorParameterValue` _output_get "Water Gradient - Bottom" (`KismetMathLibrary.HSVToRGB` 100.0 1.0 50.0 0.5))))
  (`PrimitiveComponent.SetMaterial` (`self.LiquidMesh`) 0 (`self.DynamicLiquidMaterial`))
  (`SceneComponent.SetRelativeScale3D` (`self.LiquidMesh`) (`self.StartLiquidScale`)))