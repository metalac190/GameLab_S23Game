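; BPC_CineCamSeq is a player helper that plays a cinematic level sequence while player input is suspended.
; BeginCineCameraSequence starts the given sequence player, disables input on player 0's pawn, and returns a duration from playback end frame divided by display rate numerator.
; The CineCamera graph waits that duration with a Delay, then calls EnableInput, relying on timing rather than a finished event.
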(fn `BeginCineCameraSequence`
  (params (SequencePlayer :type "MovieSceneSequencePlayer Object Reference"))
  (returns (DelayTime :type "Float (double-precision)") (PlayerPawn :type "Pawn Object Reference") (PlayerController :type "PlayerController Object Reference"))
  (bind _returnvalue (`GameplayStatics.GetPlayerPawn` 0))
  (bind _returnvalue_2 (`GameplayStatics.GetPlayerController` 0))
  (`MovieSceneSequencePlayer.Play` SequencePlayer)
  (`Actor.DisableInput` _returnvalue _returnvalue_2)
  (bind _returnvalue_3 (`MovieSceneSequenceExtensions.GetPlaybackEnd` (`MovieSceneSequencePlayer.GetSequence` (`local.SequencePlayer`))))
  (bind _returnvalue_4 (`MovieSceneSequenceExtensions.GetDisplayRate` (`MovieSceneSequencePlayer.GetSequence` (`local.SequencePlayer`))))
  (return (`KismetMathLibrary.Conv_IntToDouble` (/ _returnvalue_3 (`KismetMathLibrary.BreakFrameRate` _returnvalue_4))) _returnvalue _returnvalue_2))