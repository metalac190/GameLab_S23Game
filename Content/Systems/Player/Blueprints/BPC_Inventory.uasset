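; Player inventory component that stores items in a fixed four-slot array built on BeginPlay.
; AddToInventory writes the new item into the first slot with an empty name, returning false when all slots are full.
; On success it casts the owner to BP_Player and updates that slot in the inventory widget.
; GetStoredItem returns a slot's item with a flag for whether it is occupied.
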(event `self.ReceiveBeginPlay`
  (set `self.Inventory` (`|MakeArray` (`self.Slot1`) (`self.Slot2`) (`self.Slot3`) (`self.Slot4`))))

(fn `Add to Inventory`
  (params (NewItem :type "/Game/Entities/Gameplay/Items/S_ItemData Structure (by ref)"))
  (returns (ItemAdded :type Boolean))
  (bind _inventory (`self.Inventory`))
  (for (_array_element _array_index) _inventory
    (if (`KismetStringLibrary.IsEmpty` (`.ItemName_2_CD23B635439CECA1569C62A2D3CDE386` (break `/Game/Entities/Gameplay/Items/S_ItemData` _array_element)))
      (break)
      (elif (== _array_index (- (`KismetArrayLibrary.Array_Length` _inventory) 1))
        (return false))))
  (bind _output_get (set `self.FirstEmptySlotIndex` _array_index))
  (`|VariableSetRef` (`|GetArrayItem` _inventory _output_get) NewItem)
  (bind _asbp_player (cast `/Game/Systems/Player/Blueprints/BP_Player` (`self.GetOwner`))
    (:`then`
      (`/Game/UI/HUDs/WB_InventoryWidget.AddItemToUI` (`/Game/Systems/Player/Blueprints/BP_Player.InventoryWidget` _asbp_player) (`.ItemName_2_CD23B635439CECA1569C62A2D3CDE386` (break `/Game/Entities/Gameplay/Items/S_ItemData` NewItem)) (`self.FirstEmptySlotIndex`))
      (return true))
    (:`CastFailed`
      (`KismetSystemLibrary.PrintText` "Cast to BP_Player failed"))))

(fn `GetStoredItem`
  (params (ItemIndex :type Integer))
  (returns (ItemFound :type Boolean) (StoredItem :type "/Game/Entities/Gameplay/Items/S_ItemData Structure"))
  (bind _output (`|GetArrayItem` (`self.Inventory`) ItemIndex))
  (if (not (`KismetStringLibrary.IsEmpty` (`.ItemName_2_CD23B635439CECA1569C62A2D3CDE386` (break `/Game/Entities/Gameplay/Items/S_ItemData` _output))))
    (return true _output)
    (else
      (return false))))