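; Player component for a collectible storybook held in the first-person hands, which can be picked up, opened and flipped through.
; On BeginPlay it creates dynamic page materials on fixed hand-mesh slots, builds page info from a DataTable, restores found pages from the game instance and creates the UI widget.
; Unfound pages show a placeholder image.
; Flipping moves by two-page spreads up to the last known page, with a cooldown, and notifies listeners through dispatchers.
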(event `self.ReceiveBeginPlay`
  (`|ExecutionSequence`
    (:`then_0`
      ;[0.5521 0 0] Dynamic Storybook Page Materials (VERY IMPORTANT STATIC VALUES THAT CAN EASILY GET MESSED UP -- REFER TO FirstPerson_Hands FOR MATERIAL INDEXES)
      (bind _asbp_player (cast `/Game/Entities/Player/BP_Player` (`GameplayStatics.GetPlayerPawn` 0)))
      (bind _firstperson_hands (`/Game/Entities/Player/BP_Player.FirstPerson_Hands` _asbp_player))
      (bind _returnvalue (`PrimitiveComponent.CreateDynamicMaterialInstance` _firstperson_hands 12 "/Game/Art/_Global/First_Person_Hands/Storybook/MM_StorybookPage.MM_StorybookPage" "None"))
      (`/Engine/EditorBlueprintResources/StandardMacros.IsValid` _returnvalue
        (:`Is Valid`
          (bind _output_get (set `self.M_NextPageFlip` _returnvalue))
          (`PrimitiveComponent.SetMaterial` _firstperson_hands 12 _output_get))
        (:`Is Not Valid`
          (`KismetSystemLibrary.PrintString` "Error: Cound Not Convert Material Next Page Flip")))
      (bind _returnvalue_2 (`PrimitiveComponent.CreateDynamicMaterialInstance` _firstperson_hands 17 "/Game/Art/_Global/First_Person_Hands/Storybook/MM_StorybookPage.MM_StorybookPage" "None"))
      (`/Engine/EditorBlueprintResources/StandardMacros.IsValid` _returnvalue_2
        (:`Is Valid`
          (bind _output_get_2 (set `self.M_NextPageStatic` _returnvalue_2))
          (`PrimitiveComponent.SetMaterial` _firstperson_hands 17 _output_get_2))
        (:`Is Not Valid`
          (`KismetSystemLibrary.PrintString` "Error: Cound Not Convert Material Next Page Static")))
      (bind _returnvalue_3 (`PrimitiveComponent.CreateDynamicMaterialInstance` _firstperson_hands 13 "/Game/Art/_Global/First_Person_Hands/Storybook/MM_StorybookPage.MM_StorybookPage" "None"))
      (`/Engine/EditorBlueprintResources/StandardMacros.IsValid` _returnvalue_3
        (:`Is Valid`
          (bind _output_get_3 (set `self.M_PrevPageFlip` _returnvalue_3))
          (`PrimitiveComponent.SetMaterial` _firstperson_hands 13 _output_get_3))
        (:`Is Not Valid`
          (`KismetSystemLibrary.PrintString` "Error: Cound Not Convert Material Prev Page Flip")))
      (bind _returnvalue_4 (`PrimitiveComponent.CreateDynamicMaterialInstance` _firstperson_hands 18 "/Game/Art/_Global/First_Person_Hands/Storybook/MM_StorybookPage.MM_StorybookPage" "None"))
      (`/Engine/EditorBlueprintResources/StandardMacros.IsValid` _returnvalue_4
        (:`Is Valid`
          (bind _output_get_4 (set `self.M_PrevPageStatic` _returnvalue_4))
          (`PrimitiveComponent.SetMaterial` _firstperson_hands 18 _output_get_4))
        (:`Is Not Valid`
          (`KismetSystemLibrary.PrintString` "Error: Cound Not Convert Material Prev Page Static"))))
    (:`then_1`
      ;[1 1 1] Parse datatable to populate pageInfoMap
      (bind _outrownames (`DataTableFunctionLibrary.GetDataTableRowNames` (`self.DTStorybook`)))
      (set `self.storybookLength` (`KismetArrayLibrary.Array_Length` _outrownames))
      (for (_array_element _array_index) _outrownames
        (bind _returnvalue_5 (`|GetDataTableRow` "/Game/Data/StorybookPages.StorybookPages" _array_element)
          (:`then`
            (`BlueprintMapLibrary.Map_Add` (`self.pageInfoMap`) _array_element (make `/Game/Systems/Structures/Storybook/PageInfo` _array_element (`.Image_3_7B6234204F03C062D2C19992E7992FD0` (break `/Game/Systems/Structures/Storybook/PageImage` _returnvalue_5)) (+ _array_index 1))))))
      (bind _assave_game_instance (cast `/Game/Systems/Saves/SaveGameInstance` (`GameplayStatics.GetGameInstance`)))
      (bind _output_get_5 (set `self.As Save Game Instance` _assave_game_instance))
      (bind _pagesfound (`/Game/Systems/Saves/SaveGameInstance.LoadPages` _output_get_5))
      (`self.LoadPages` _pagesfound))
    (:`then_2`
      ;[1 1 1] Initilaize Widget
      (bind _returnvalue_6 (`|CreateWidget` "/Game/UI/Widgets/StorybookUI.StorybookUI_C" (`GameplayStatics.GetPlayerController` 0)))
      (set `self.widget` _returnvalue_6))
    (:`then_3`
      (set `self.CanFlipPage` true))))

(event `PickupStorybook`
  ;[1 0.4611 0] Storybook Pickup Animation of 7.5 Seconds
  (`self.StorybookPickup`)
  (`KismetSystemLibrary.Delay` 7.5)
  (set `self.hasBook` true))

(event `ToggleStorybook`
  (if (`self.hasBook`)
    (if (`self.isOpen`)
      (`Widget.RemoveFromParent` (`self.widget`))
      (set `self.isOpen` false)
      (`GameplayStatics.PlaySound2D` "/Game/Audio/Gameplay/waves/sfx_book_close_01.sfx_book_close_01" 1.0 1.0 0.0 null null)
      (else
        (`UserWidget.AddToViewport` (`self.widget`) 0)
        (set `self.isOpen` true)
        (`KismetSystemLibrary.Delay` 0.2)
        (`GameplayStatics.PlaySound2D` "/Game/Audio/Gameplay/Cues/sfx_book_open_01.sfx_book_open_01" 1.0 1.0 0.0 null null)))
    (`self.StorybookToggled` (`self.isOpen`))
    (`/Game/UI/Widgets/StorybookUI.Set Buttons to Correct System` (`self.widget`))
    (else
      (`KismetSystemLibrary.PrintString` "Haven't collected storybook"))))

(event `Add Page`
  (params (`Page Name` :type Name) (`Other Pages` :type "Array of Name"))
  (`BlueprintSetLibrary.Set_Add` (`self.pagesFound`) `Page Name`)
  (`BlueprintSetLibrary.Set_AddItems` (`self.pagesFound`) `Other Pages`)
  (`self.UpdateCurrentPage` `Page Name`)
  (`GameplayStatics.PlaySound2D` "/Game/Audio/Gameplay/Cues/sfx_book_addPage.sfx_book_addPage" 1.0 1.0 0.0 null null)
  (`self.SetLastKnownPage`)
  (`/Game/Systems/Saves/SaveGameInstance.SavePages` (`self.As Save Game Instance`) (`self.pagesFound`)))

(event `Flip Page Right`
  (if (and (`self.isOpen`) (`self.CanFlipPage`))
    (if (not (== (`self.current page`) 0))
      (set `self.current page` (- (`self.current page`) 2))
      (`self.UpdateActivePage` self true)
      (`GameplayStatics.PlaySound2D` "/Game/Audio/Gameplay/Cues/sfx_book_pageTurn.sfx_book_pageTurn" 1.0 1.0 0.0 null null :!label _label)
      (set `self.CanFlipPage` false)
      (`KismetSystemLibrary.Delay` (`self.FlipCooldown`))
      (set `self.CanFlipPage` true))))

(event `Flip Page Left`
  (if (and (`self.isOpen`) (`self.CanFlipPage`))
    (if (< (`self.current page`) (- (`self.lastPageKnown`) 2))
      (set `self.current page` (+ (`self.current page`) 2))
      (`self.UpdateActivePage` self)
      (goto _label))))

(fn `Get_Page_Info`
  (params (index :type Integer))
  (returns (PageInfo :type "/Game/Systems/Structures/Storybook/PageInfo Structure"))
  (locals (Image :type "Texture2D Object Reference"))
  (bind _pageinfomap (`self.pageInfoMap`))
  (bind _keys (`BlueprintMapLibrary.Map_Keys` _pageinfomap))
  (bind _value (`BlueprintMapLibrary.Map_Find` _pageinfomap (`|GetArrayItem` _keys index)))
  (if (not (`BlueprintSetLibrary.Set_Contains` (`self.pagesFound`) (break `/Game/Systems/Structures/Storybook/PageInfo` _value)))
    (set `local.Image` (`self.404Page`))
    (else
      (set `local.Image` (`.Image_13_AF2B684340CCA38086B91596DD7403E0` (break `/Game/Systems/Structures/Storybook/PageInfo` _value)))))
  (return (make `/Game/Systems/Structures/Storybook/PageInfo` (break `/Game/Systems/Structures/Storybook/PageInfo` _value) (`local.Image`) (`.PageNumber_12_4B6AB89142DF46561D6F178EA88DBB30` (break `/Game/Systems/Structures/Storybook/PageInfo` _value)))))

(fn `LoadPages`
  (params (pagesFound :type "Set of Name"))
  (bind _result (`BlueprintSetLibrary.Set_ToArray` pagesFound))
  (`BlueprintSetLibrary.Set_AddItems` (`self.pagesFound`) _result)
  (`self.SetLastKnownPage`))

(fn `SavePages`
  (returns (pagesFound :type "Set of Name"))
  (return (`self.pagesFound`)))

(fn `SetLastKnownPage`
  (bind _result (`BlueprintSetLibrary.Set_ToArray` (`self.pagesFound`)))
  (for _array_element _result
    (set `self.lastPageKnown` (`KismetMathLibrary.Max` (`.PageNumber_12_4B6AB89142DF46561D6F178EA88DBB30` (break `/Game/Systems/Structures/Storybook/PageInfo` (`BlueprintMapLibrary.Map_Find` (`self.pageInfoMap`) _array_element))) (`self.lastPageKnown`)))))

(fn `UpdateCurrentPage`
  (params (PageName :type Name))
  (bind (_value _returnvalue) (`BlueprintMapLibrary.Map_Find` (`self.pageInfoMap`) PageName))
  (bind _returnvalue_2 (- (`.PageNumber_12_4B6AB89142DF46561D6F178EA88DBB30` (break `/Game/Systems/Structures/Storybook/PageInfo` _value)) 1))
  (if _returnvalue
    (set `self.current page` (`KismetMathLibrary.SelectInt` _returnvalue_2 (- _returnvalue_2 1) (== (mod _returnvalue_2 2) 0)))))