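; BP_LadderNew is a spline-based ladder that switches the player's movement component in and out of a climbing mode, hiding first-person hands while climbing.
; The bottom trigger passes through a gate with a half-second reopen delay to start climbing, or reset if the mode change fails.
; The top trigger flags NearLadderEnd and restores movement on exit unless the linetrace trigger marks OnLadder.
; The construction script places MoveTypeChangeLocation at a fraction along the spline.
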(event `OpenGate`
  ;[1 1 1] Ladder Bottom
  (`KismetSystemLibrary.Delay` 0.5)
  (goto _label :!via `Open`))

(event `self.EntryTrigger.OnComponentBeginOverlap`
  (params (OverlappedComponent :type "PrimitiveComponent Object Reference") (OtherActor :type "Actor Object Reference") (OtherComp :type "PrimitiveComponent Object Reference") (OtherBodyIndex :type Integer) (bFromSweep :type Boolean) (SweepResult :type "HitResult Structure (by ref)"))
  ;[1 1 1] Ladder Bottom
  (`/Engine/EditorBlueprintResources/StandardMacros.Gate` false :!label _label
    (:`Exit`
      (bind _asbp_player (cast `/Game/Entities/Player/BP_Player` OtherActor))
      (bind _ac_movement (`/Game/Entities/Player/BP_Player.AC_Movement` _asbp_player))
      (bind _success (`/Game/Systems/Player/AC_Movement.SetMoveMode` _ac_movement "NewEnumerator2"))
      (set `/Game/Systems/Player/AC_Movement.LadderSpline` (`self.Spline`) _ac_movement)
      (`SceneComponent.SetVisibility` (`/Game/Entities/Player/BP_Player.FirstPerson_Hands` _asbp_player) false false)
      (if _success
        (`self.Close Gate`)
        (`self.OpenGate`)
        (else
          (`/Game/Systems/Player/AC_Movement.SetMoveMode` _ac_movement "NewEnumerator0")
          (set `/Game/Systems/Player/AC_Movement.LadderSplinePos` 0.0 _ac_movement)
          (`SceneComponent.SetVisibility` (`/Game/Entities/Player/BP_Player.FirstPerson_Hands` _asbp_player) true false))))))

(event `Close Gate`
  ;[1 1 1] Ladder Bottom
  (goto _label :!via `Close`))

(event `self.ExitTrigger.OnComponentEndOverlap`
  (params (OverlappedComponent :type "PrimitiveComponent Object Reference") (OtherActor :type "Actor Object Reference") (OtherComp :type "PrimitiveComponent Object Reference") (OtherBodyIndex :type Integer))
  ;[1 1 1] Ladder Top
  (if (not (`self.OnLadder`))
    (bind _asbp_player (cast `/Game/Entities/Player/BP_Player` OtherActor))
    (bind _ac_movement (`/Game/Entities/Player/BP_Player.AC_Movement` _asbp_player))
    (set `/Game/Systems/Player/AC_Movement.NearLadderEnd` false _ac_movement)
    (bind _mode (`/Game/Systems/Player/AC_Movement.GetMoveMode` _ac_movement))
    (if (`|EnumEquality` _mode "NewEnumerator2")
      (`/Game/Systems/Player/AC_Movement.SetMoveMode` _ac_movement "NewEnumerator0")
      (set `/Game/Systems/Player/AC_Movement.LadderSplinePos` 0.0 _ac_movement)
      (`SceneComponent.SetVisibility` (`/Game/Entities/Player/BP_Player.FirstPerson_Hands` _asbp_player) true false))))

(event `self.LinetraceTrigger.OnComponentBeginOverlap`
  (params (OverlappedComponent :type "PrimitiveComponent Object Reference") (OtherActor :type "Actor Object Reference") (OtherComp :type "PrimitiveComponent Object Reference") (OtherBodyIndex :type Integer) (bFromSweep :type Boolean) (SweepResult :type "HitResult Structure (by ref)"))
  ;[1 1 1] Track Proximity to Ladder
  (cast `/Game/Entities/Player/BP_Player` OtherActor)
  (set `self.OnLadder` true))

(event `self.LinetraceTrigger.OnComponentEndOverlap`
  (params (OverlappedComponent :type "PrimitiveComponent Object Reference") (OtherActor :type "Actor Object Reference") (OtherComp :type "PrimitiveComponent Object Reference") (OtherBodyIndex :type Integer))
  ;[1 1 1] Track Proximity to Ladder
  (cast `/Game/Entities/Player/BP_Player` OtherActor)
  (set `self.OnLadder` false))

(event `self.ExitTrigger.OnComponentBeginOverlap`
  (params (OverlappedComponent :type "PrimitiveComponent Object Reference") (OtherActor :type "Actor Object Reference") (OtherComp :type "PrimitiveComponent Object Reference") (OtherBodyIndex :type Integer) (bFromSweep :type Boolean) (SweepResult :type "HitResult Structure (by ref)"))
  ;[1 1 1] Track Proximity to Ladder
  (bind _asbp_player (cast `/Game/Entities/Player/BP_Player` OtherActor))
  (set `/Game/Systems/Player/AC_Movement.NearLadderEnd` true (`/Game/Entities/Player/BP_Player.AC_Movement` _asbp_player)))

(fn `UserConstructionScript`
  (bind _spline (`self.Spline`))
  (`SceneComponent.K2_SetWorldLocation` (`self.MoveTypeChangeLocation`) (`SplineComponent.GetLocationAtDistanceAlongSpline` _spline (* (`SplineComponent.GetSplineLength` _spline) (`self.SpeedChangeDistance`)) "World") true true))