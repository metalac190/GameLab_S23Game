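; BP_Crafter is an interactable crafting station that combines items from the player's inventory.
; Each Interact performs one step: collect any output, craft when inputs are full, or deposit the equipped item.
; BPCCrafter holds the items and does the crafting, exchanging them with the player's BPCInventory.
; SetMeshes mirrors its contents on two input spots and an output spot, while UseWith sets the displayed text.
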(event `/Game/Systems/Mechanics/BP_InteractableInterface.Interact`
  (params (Player :type "/Game/Entities/Player/Blueprints/BP_Player Object Reference"))
  (bind _bp_player (`self.BP_Player`))
  (bind _bpc_crafter (`self.BPC_Crafter`))
  (bind _output_item_itemname (break `/Game/Entities/Gameplay/Items/S_ItemData` (`/Game/Systems/Mechanics/Crafting/BPC_Crafter.Output Item` (`self.BPC_Crafter`))))
  (bind _equippedindex (`/Game/Entities/Player/Blueprints/BP_Player.EquippedIndex` _bp_player))
  (bind _asbp_player (cast `/Game/Entities/Player/Blueprints/BP_Player` (`GameplayStatics.GetPlayerPawn` 0)))
  (set `self.BP_Player` _asbp_player)
  (if (not (`KismetStringLibrary.IsEmpty` _output_item_itemname))
    (`/Game/Entities/Player/Blueprints/BPC_Inventory.AddToInventory` (`/Game/Entities/Player/Blueprints/BP_Player.BPC_Inventory` (`self.BP_Player`)) (`/Game/Systems/Mechanics/Crafting/BPC_Crafter.Output Item` (`self.BPC_Crafter`)))
    (`self.SetMeshes`)
    (elif (== (`KismetArrayLibrary.Array_Length` (`/Game/Systems/Mechanics/Crafting/BPC_Crafter.Input Items` _bpc_crafter)) (`/Game/Systems/Mechanics/Crafting/BPC_Crafter.Max Items` _bpc_crafter))
      (`/Game/Systems/Mechanics/Crafting/BPC_Crafter.Craft` (`self.BPC_Crafter`))
      (`self.SetMeshes`)
      (elif (>= _equippedindex 0)
        (bind (_itemfound _storeditem) (`/Game/Entities/Player/Blueprints/BPC_Inventory.GetStoredItem` (`/Game/Entities/Player/Blueprints/BP_Player.BPC_Inventory` _bp_player) _equippedindex))
        (if _itemfound
          (`/Game/Systems/Mechanics/Crafting/BPC_Crafter.Add Item` (`self.BPC_Crafter`) _storeditem)
          (`/Game/Entities/Player/Blueprints/BP_Player.RemoveEquippedItem` (`self.BP_Player`))
          (`self.SetMeshes`)
          (else
            (`KismetSystemLibrary.PrintString` "Item Can't be crafted with!")))))))

(fn `SetMeshes`
  (locals (mesh :type "StaticMeshComponent Object Reference"))
  (bind (_output_item_itemname _output_item_itemmesh) (break `/Game/Entities/Gameplay/Items/S_ItemData` (`/Game/Systems/Mechanics/Crafting/BPC_Crafter.Output Item` (`self.BPC_Crafter`))))
  (`StaticMeshComponent.SetStaticMesh` (`self.Input Spot 1`) null)
  (`StaticMeshComponent.SetStaticMesh` (`self.Input Spot 2`) null)
  (for (_array_element _array_index) (`/Game/Systems/Mechanics/Crafting/BPC_Crafter.Input Items` (`self.BPC_Crafter`))
    (switch `int` _array_index
      (:`0`
        (set `local.mesh` (`self.Input Spot 1`)))
      (:`1`
        (bind _output_get (set `local.mesh` (`self.Input Spot 2`)))))
    (`StaticMeshComponent.SetStaticMesh` _output_get (`.ItemMesh_12_7EE7D8D84E9FEE43260F5A97623E8EBD` (break `/Game/Entities/Gameplay/Items/S_ItemData` _array_element)))
    (`StaticMeshComponent.SetStaticMesh` (`self.Output Spot`) _output_item_itemmesh)))

(fn `UserConstructionScript`)

(fn `UseWith`
  (params (ObjectToUse :type "Actor Object Reference") (`Text To Show` :type Text))
  (returns (ObjectReturned :type "Actor Object Reference"))
  (`TextRenderComponent.K2_SetText` (`self.text`) `Text To Show`))