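; Crafting component that collects allowed items up to a limit and crafts them on demand or when full.
; Matches input names against a recipe DataTable, ordered or unordered, briefly spawning the output actor to read its item data.
; Each attempt clears inputs and frees matching level item sources.
; Results go to player inventory or back into the input, except final items, which replace the equipped item; flint & steel also notifies the player.
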(event `self.ReceiveBeginPlay`
  (bind _outactors (`GameplayStatics.GetAllActorsOfClass` "/Game/Entities/Gameplay/Items/BP_ItemSource.BP_ItemSource_C"))
  (set `self.ItemSources` _outactors))

(event `Craft`
  (params (AutoEquip :type Boolean))
  (bind _input_items (`self.Input Items`))
  (bind _returnvalue (`Actor.K2_GetActorLocation` (`GameplayStatics.GetPlayerPawn` 0)))
  (bind _names (`self.GetNamesFromItemData` (`self.Input Items`)))
  (bind (_output_item _recipe_used) (`self.CraftFromRecipe` _names))
  (`self.ResetItemSources` _input_items)
  (`KismetArrayLibrary.Array_Clear` _input_items)
  (`self.ItemCrafted` _output_item)
  (if (not (`KismetStringLibrary.IsEmpty` (`.ItemName_18_CD23B635439CECA1569C62A2D3CDE386` (break `/Game/Entities/Gameplay/Items/S_ItemData` _output_item))))
    (bind _output_get (set `self.Output Item` _output_item))
    (bind _itemname (break `/Game/Entities/Gameplay/Items/S_ItemData` _output_get))
    (if (== _itemname "flint & steel")
      (bind _asbp_player (cast `/Game/Entities/Player/BP_Player` (`GameplayStatics.GetPlayerPawn` 0))
        (:`then`
          (`/Game/Entities/Player/BP_Player.CraftFlintNSteel` _asbp_player))
        (:`CastFailed`
          _)))
    (`GameplayStatics.PlaySoundAtLocation` (`.SFX_25_1BAB5F6149906158BF072B9BAB0752B5` (break `/Game/Systems/Mechanics/Crafting/Recipe` _recipe_used)) _returnvalue (struct) 1.0 1.0 0.0 null null null null)
    (`KismetSystemLibrary.PrintString` (`KismetStringLibrary.Concat_StrStr` "Crafted " _itemname))
    (bind _crafteritemreplaced (`self.CheckFinalItem`))
    (if (not _crafteritemreplaced)
      ;[1 1 1] Manage Output
      (switch `/Game/Systems/Mechanics/Crafting/OutputMode` (`self.OutputMode`)
        (:`NewEnumerator0`
          (bind _asbp_player_2 (cast `/Game/Entities/Player/BP_Player` (`GameplayStatics.GetPlayerPawn` 0)))
          (bind (_itemadded _index) (`/Game/Systems/Player/BPC_Inventory.AddToInventory` (`/Game/Entities/Player/BP_Player.BPC_Inventory` _asbp_player_2) (`self.Output Item`)))
          (if _itemadded
            (if AutoEquip
              (`/Game/Entities/Player/BP_Player.EquipItem` _asbp_player_2 _index))
            (set `self.Output Item` (struct) :!label _label)))
        (:`NewEnumerator1`
          (bind _itemadded_2 (`self.Add Item` (`self.Output Item`)))
          (if _itemadded_2
            (goto _label)))))
    (else
      (`GameplayStatics.PlaySoundAtLocation` "/Game/Audio/Gameplay/Cues/sfx_craftFailure_01.sfx_craftFailure_01" _returnvalue (struct) 1.0 1.0 0.0 null null null null)
      (`KismetSystemLibrary.PrintString` "Inputs did not craft anything"))))

(fn `Add Item`
  (params (ItemToAdd :type "/Game/Entities/Gameplay/Items/S_ItemData Structure (by ref)"))
  (returns (itemAdded :type Boolean))
  ;[1 1 1] Check Validity
  (bind _returnvalue (`self.IsInputFull`))
  (if _returnvalue
    (`KismetSystemLibrary.PrintString` "Inputs Full")
    (elif (`self.IsAllowed` ItemToAdd)
      (`KismetArrayLibrary.Array_Add` (`self.Input Items`) ItemToAdd)
      (`self.ItemAdded` ItemToAdd)
      ;[1 1 1] Craft if full
      (if (`self.craftWhenFull`)
        (`KismetSystemLibrary.PrintString` (`KismetStringLibrary.Concat_StrStr` "Added " (`.ItemName_18_CD23B635439CECA1569C62A2D3CDE386` (break `/Game/Entities/Gameplay/Items/S_ItemData` ItemToAdd)) " to crafting input"))
        (bind _returnvalue_2 (`self.IsInputFull`))
        (if _returnvalue_2
          (`self.Craft` false)))
      (return true)
      (else
        (`KismetSystemLibrary.PrintString` "This item can't go in this crafter"))))
  (return false))

(fn `CheckFinalItem`
  (returns (crafterItemReplaced :type Boolean))
  (bind _output_item_itemname (break `/Game/Entities/Gameplay/Items/S_ItemData` (`self.Output Item`)))
  (bind _output_item (`self.Output Item`))
  (bind _output_item_itemname_2 (break `/Game/Entities/Gameplay/Items/S_ItemData` (`self.Output Item`)))
  (bind _asbp_player (cast `/Game/Entities/Player/BP_Player` (`self.GetOwner`))
    (:`then`
      (for _array_element (`self.FinalItems`)
        (if (== _array_element _output_item_itemname_2)
          (`/Game/Entities/Player/BP_Player.RemoveEquippedItem` _asbp_player)
          (bind _bpc_inventory (`/Game/Entities/Player/BP_Player.BPC_Inventory` _asbp_player))
          (bind _itemadded (`/Game/Systems/Player/BPC_Inventory.AddToInventory` _bpc_inventory _output_item))
          (if _itemadded
            (`/Game/Entities/Player/BP_Player.EquipItem` _asbp_player (`KismetArrayLibrary.Array_Find` (`/Game/Systems/Player/BPC_Inventory.Inventory` _bpc_inventory) _output_item))
            (`KismetSystemLibrary.PrintString` (`KismetStringLibrary.Concat_StrStr` "Changed equipped item to " _output_item_itemname))
            (return true)))))
    (:`CastFailed`
      _))
  (return false))

(fn `CraftFromRecipe`
  (params (Inputs :type "Array of Name"))
  (returns (`Output Item` :type "/Game/Entities/Gameplay/Items/S_ItemData Structure") (`Recipe Used` :type "/Game/Systems/Mechanics/Crafting/Recipe Structure"))
  (locals (outputItemData :type "/Game/Entities/Gameplay/Items/S_ItemData Structure"))
  (bind _outrownames (`DataTableFunctionLibrary.GetDataTableRowNames` (`self.Recipe DataTable`)))
  (for _array_element _outrownames
    (bind _returnvalue (`|GetDataTableRow` (`self.Recipe DataTable`) _array_element)
      (:`then`
        (bind (_sourceitems _outputitem _forceorder) (break `/Game/Systems/Mechanics/Crafting/Recipe` _returnvalue))
        (bind _is_recipe (`self.IsRecipe` Inputs _sourceitems _forceorder))
        (if _is_recipe
          (bind _returnvalue_2 (`|SpawnActorFromClass` _outputitem (`KismetMathLibrary.MakeTransform` (0.0 0.0 0.0)) "Undefined" "OverrideRootScale" null null))
          (set `local.outputItemData` (`/Game/Entities/Gameplay/Items/BP_ITEM_MASTER.ItemData` _returnvalue_2))
          (`Actor.K2_DestroyActor` _returnvalue_2)
          (return (`local.outputItemData`) _returnvalue)))))
  (return))

(fn `GetNamesFromItemData`
  (params (ItemData :type "Array of /Game/Entities/Gameplay/Items/S_ItemData Structure"))
  (returns (Names :type "Array of Name"))
  (locals (localNames :type "Array of Name"))
  (for _array_element ItemData
    (`KismetArrayLibrary.Array_Add` (`local.localNames`) (`KismetStringLibrary.Conv_StringToName` (break `/Game/Entities/Gameplay/Items/S_ItemData` _array_element))))
  (return (`local.localNames`)))

(fn `IsInputFull`
  (returns (ReturnValue :type Boolean))
  (return (>= (`KismetArrayLibrary.Array_Length` (`self.Input Items`)) (`self.Max Items`))))

(fn `IsRecipe`
  (params (Inputs :type "Array of Name") (Recipe :type "Array of Name") (`Order matters` :type Boolean))
  (returns (`is recipe` :type Boolean))
  (locals (Items :type "Set of Name") (Matches :type Boolean :default true))
  (if (== (`KismetArrayLibrary.Array_Length` Inputs) (`KismetArrayLibrary.Array_Length` Recipe))
    (if `Order matters`
      (return (`KismetArrayLibrary.Array_Identical` Inputs Recipe))
      (else
        ;[1 1 1] Find if items match unordered
        (`BlueprintSetLibrary.Set_AddItems` (`local.Items`) Recipe)
        (set `local.Matches` true)
        (for _array_element Inputs
          (if (`BlueprintSetLibrary.Set_Contains` (`local.Items`) _array_element)
            (`BlueprintSetLibrary.Set_Remove` (`local.Items`) _array_element)
            (else
              (set `local.Matches` false)
              (break))))
        (return (`local.Matches`))))
    (else
      (return false))))

(fn `ResetItemSources`
  (params (Items :type "Array of /Game/Entities/Gameplay/Items/S_ItemData Structure"))
  (locals (names :type "Set of String"))
  (for _array_element Items
    (`BlueprintSetLibrary.Set_Add` (`local.names`) (break `/Game/Entities/Gameplay/Items/S_ItemData` _array_element)))
  (for _array_element_2 (`self.ItemSources`)
    (bind _itemdata_itemname (break `/Game/Entities/Gameplay/Items/S_ItemData` (`/Game/Entities/Gameplay/Items/BP_ItemSource.ItemData` _array_element_2)))
    (if (`BlueprintSetLibrary.Set_Contains` (`local.names`) _itemdata_itemname)
      (bind _output_get (set `/Game/Entities/Gameplay/Items/BP_ItemSource.ItemInUse` false _array_element_2))
      (`KismetSystemLibrary.PrintString` (`KismetStringLibrary.Concat_StrStr` "set itemInUse to " (`KismetStringLibrary.Conv_BoolToString` _output_get) " for " (`KismetSystemLibrary.GetDisplayName` _array_element_2))))))