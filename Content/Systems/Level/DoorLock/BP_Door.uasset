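; BP_Door is an interactable door actor that can require keys to open.
; When locked, Interact matches the player's equipped item name against the first Keys entry, optionally consumes it, and opens once the list is empty.
; OpenDoor currently destroys the actor, leaving the pivot rotation timeline unconnected.
; GetPrompt supplies unlock text based on the equipped item, regardless of lock state.
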(event `self.ReceiveBeginPlay`
  (set `self.DoorOpen` false))

(event `/Game/Systems/Mechanics/BP_InteractableInterface.Interact`
  (params (Player :type "/Game/Entities/Player/Blueprints/BP_Player Object Reference"))
  ;[1 1 1] Interact -- Hook up to Player Interactable Interface Eventually
  (if (`self.DoorOpen`)
    _
    (elif (`self.Locked`)
      (bind _unlocked (`self.TryUnlock` Player))
      (if _unlocked
        (`self.OpenDoor`))
      (else
        (`self.OpenDoor`)))))

(event `OpenDoor`
  ;[1 1 1] Open Door
  (`self.K2_DestroyActor`))

(fn `Get Prompt`
  (params (player :type "/Game/Entities/Player/Blueprints/BP_Player Object Reference"))
  (returns (inputAction :type "InputAction Object Reference") (actionText :type Text))
  (bind (_itemequipped _equippeditem) (`/Game/Entities/Player/Blueprints/BP_Player.GetEquippedItem` player))
  (if _itemequipped
    (return "/Game/Entities/Player/Input/Actions/IA_Interact.IA_Interact" (`KismetTextLibrary.Conv_StringToText` (`KismetStringLibrary.Concat_StrStr` "unlock with " (break `/Game/Entities/Gameplay/Items/S_ItemData` _equippeditem))))
    (else
      (return null "Equip an item to unlock"))))

(fn `SetLocked`
  (params (Locked :type Boolean))
  (set `self.Locked` Locked))

(fn `TryUnlock`
  (params (NewParam :type "/Game/Entities/Player/Blueprints/BP_Player Object Reference"))
  (returns (unlocked :type Boolean))
  (bind _keys (`self.Keys`))
  (if (`KismetArrayLibrary.Array_IsEmpty` (`self.Keys`))
    (return true)
    (else
      (bind (_itemequipped _equippeditem) (`/Game/Entities/Player/Blueprints/BP_Player.GetEquippedItem` NewParam))
      (if _itemequipped
        (if (== (break `/Game/Entities/Gameplay/Items/S_ItemData` _equippeditem) (`|GetArrayItem` (`self.Keys`)))
          (`KismetSystemLibrary.PrintString` "Used Key to unlock")
          (if (`self.eatKey`)
            (`/Game/Entities/Player/Blueprints/BP_Player.RemoveEquippedItem` NewParam))
          (`KismetArrayLibrary.Array_Remove` _keys)
          (return (`KismetArrayLibrary.Array_IsEmpty` _keys))
          (else
            _)))
      (`KismetSystemLibrary.PrintString` "Key doesn't unlock")
      (return false))))

(fn `UserConstructionScript`)