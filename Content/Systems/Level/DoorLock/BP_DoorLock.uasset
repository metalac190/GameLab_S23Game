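; BP_DoorLock is a level actor that keeps a referenced door locked until the lock is melted.
; It locks the door on BeginPlay, and Interact triggers MeltLock, though the acid check is only a debug print and the interaction interface is not yet hooked up.
; A timeline scales the lock's root each update, then unlocks the door and destroys the actor when finished.
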(event `self.ReceiveBeginPlay`
  (`/Game/Systems/Level/DoorLock/BP_Door.SetLocked` (`self.Door`) true))

(event `Interact`
  ;[1 1 1] Interact -- Hook up to Player Interactable Interface Eventually
  (`KismetSystemLibrary.PrintString` "Check Player Holding Acid")
  (`self.MeltLock`))

(event `MeltLock`
  ;[1 1 1] Melt Lock
  (bind (_direction _scaletrack) (`Timeline|MeltLockTimeline`)
    (:`Update`
      (`SceneComponent.SetWorldScale3D` (`self.DefaultSceneRoot`) (`KismetMathLibrary.Conv_DoubleToVector` _scaletrack)))
    (:`Finished`
      (`/Game/Systems/Level/DoorLock/BP_Door.SetLocked` (`self.Door`) false)
      (`self.K2_DestroyActor`))))

(fn `UserConstructionScript`)