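; BP_HideSequence runs a timed hiding challenge that checks whether the player is hidden when time runs out.
; It can start on BeginPlay or by event, waits for the sequence length, then polls its array of valid hiding volumes for any reporting the player hidden.
; Success and failure branch into separate events, which currently only print debug messages for level notification and player death.
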(event `self.ReceiveBeginPlay`
  (if (`self.AutoStartHideSequence`)
    (`self.StartHideSequence`)))

(event `StartHideSequence`
  (`KismetSystemLibrary.PrintString` "BeginHidingSequence")
  (`KismetSystemLibrary.Delay` (`self.SequenceLength`))
  (`self.CheckPlayerHidden`)
  (if (`self.PlayerHidden`)
    (`self.PlayerSuccessfullyHidden`)
    (else
      (`self.PlayerNotHidden`))))

(event `PlayerSuccessfullyHidden`
  (`KismetSystemLibrary.PrintString` "Hidden Successfully, Notify Level Blueprint"))

(event `PlayerNotHidden`
  (`KismetSystemLibrary.PrintString` "Death -- Player Not Hidden"))

(fn `CheckPlayerHidden`
  (`|ExecutionSequence`
    (:`then_0`
      (set `self.PlayerHidden` false))
    (:`then_1`
      (for _array_element (`self.ValidVolumes`)
        (if (`/Game/Systems/Level/Hiding/BP_HideVolume.PlayerHidden` _array_element)
          (set `self.PlayerHidden` true))))))

(fn `UserConstructionScript`)