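; BP_Moondial is an interactable moondial that opens sets of vine doors as the player presents moon phase items in sequence.
; On Interact, it switches on the current Phase and checks the player's equipped item by name against the next moon phase.
; A match opens every vine door in that phase's array and advances Phase, enforcing the order through all four phases.
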(event `/Game/Systems/Mechanics/BP_InteractableInterface.Interact`
  (params (Player :type "/Game/Entities/Player/Blueprints/BP_Player Object Reference"))
  (bind _equippeditem_itemname (break `/Game/Entities/Gameplay/Items/S_ItemData` (`/Game/Entities/Player/Blueprints/BP_Player.EquippedItem` Player)))
  (switch `int` (`self.Phase`)
    (:`0`
      (if (== _equippeditem_itemname "Moon Phase 1")
        (`self.OpenVineDoors` (`self.Phase1Doors`))
        (set `self.Phase` 1)))
    (:`1`
      (if (== _equippeditem_itemname "Moon Phase 2")
        (`self.OpenVineDoors` (`self.Phase2Doors`))
        (set `self.Phase` 2)))
    (:`2`
      (if (== _equippeditem_itemname "Moon Phase 3")
        (`self.OpenVineDoors` (`self.Phase3Doors`))
        (set `self.Phase` 3)))
    (:`3`
      (if (== _equippeditem_itemname "Moon Phase 4")
        (`self.OpenVineDoors` (`self.Phase4Doors`))
        (set `self.Phase` 4)))))

(fn `OpenVineDoors`
  (params (NewParam :type "Array of /Game/Systems/Level/Vines/BP_VineDoor Object Reference"))
  (for _array_element NewParam
    (`/Game/Systems/Level/Vines/BP_VineDoor.OpenVineDoor` _array_element)))

(fn `UserConstructionScript`)