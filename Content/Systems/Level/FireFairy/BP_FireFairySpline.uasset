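; Fire fairy spline actor that plays a particle effect with configurable color, size and path travel duration.
; BeginPlay deactivates the effect, then calls StartEffect if PlayOnAwake is set, optionally after a delay.
; StartEffect binds itself to the fairy event dispatcher, then activates the effect and sets its parameters.
; Tick adds a sine-based vertical offset to the spline each frame for a hovering motion.
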(event `StartEffect`
  (bind _fx_firefairy (`self.FX_FireFairy`))
  (add `self.FairyEventDispatcher` (delegate `StartEffect`))
  (`ActorComponent.Activate` _fx_firefairy true)
  (`NiagaraComponent.SetVariableLinearColor` _fx_firefairy "Color" (`self.ParticleColor`))
  (`NiagaraComponent.SetVariableFloat` _fx_firefairy "Loop Duration" (`self.PathTravelDuration`))
  (`NiagaraComponent.SetVariableFloat` _fx_firefairy "ParticleSize" (`self.ParticleSize`)))

(event `self.ReceiveBeginPlay`
  (`ActorComponent.Deactivate` (`self.FX_FireFairy`))
  (if (`self.PlayOnAwake`)
    (if (`self.hasDelay?`)
      (`KismetSystemLibrary.Delay` (`self.DelayDuration`))
      (`self.StartEffect`)
      (else
        (`self.StartEffect`)))))

(event `self.ReceiveTick`
  (params (DeltaSeconds :type "Float (single-precision)"))
  (`SceneComponent.K2_AddRelativeLocation` (`self.Spline`) (`KismetMathLibrary.MakeVector` 0.0 0.0 (* (`KismetMathLibrary.Sin` (* (`self.GetGameTimeSinceCreation`) (`self.Hover Frequency`))) (`self.Hover Amplitude`))) false false))

(fn `UserConstructionScript`)