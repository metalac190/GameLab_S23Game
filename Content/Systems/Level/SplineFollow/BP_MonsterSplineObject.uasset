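; Monster actor that travels once along a referenced spline at a set speed, hidden and without collision until activated.
; FollowSpline, run on BeginPlay if AutoActivate is set, resets distance and reveals the capsule.
; Tick moves and rotates the capsule by distance along the spline.
; At the end it hides again, disables collision and fires the CompletedSpline dispatcher, intended for the Level Blueprint.
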(event `self.ReceiveBeginPlay`
  (bind _capsulecomponent (`self.CapsuleComponent`))
  (`PrimitiveComponent.SetCollisionEnabled` _capsulecomponent "NoCollision")
  (`SceneComponent.SetHiddenInGame` _capsulecomponent true true)
  (set `self.Enabled` false)
  (if (`self.AutoActivate`)
    (`self.FollowSpline`)))

(event `self.ReceiveTick`
  (params (DeltaSeconds :type "Float (single-precision)"))
  (bind _capsulecomponent (`self.CapsuleComponent`))
  (bind _spline (`/Game/Systems/Level/SplineFollow/BP_SimpleSplineFollow.Spline` (`self.SplineRef`)))
  (if (`self.Enabled`)
    (bind _output_get (set `self.SplineDelta` (+ (`self.SplineDelta`) (* DeltaSeconds (`self.Speed`)))))
    (if (> _output_get (`SplineComponent.GetSplineLength` _spline))
      (set `self.Enabled` false)
      (`KismetSystemLibrary.PrintString` "Completed Spline. Notify Level Blueprint")
      (`self.CompletedSpline`)
      (`SceneComponent.SetHiddenInGame` _capsulecomponent true true)
      (`PrimitiveComponent.SetCollisionEnabled` _capsulecomponent "NoCollision")
      (else
        (bind (_returnvalue _returnvalue2) (`self.GetSplineLocRot` _spline _output_get))
        (`SceneComponent.K2_SetWorldLocationAndRotation` (`self.CapsuleComponent`) _returnvalue _returnvalue2 false false)))))

(event `FollowSpline`
  (bind _capsulecomponent (`self.CapsuleComponent`))
  (`/Engine/EditorBlueprintResources/StandardMacros.IsValid` (`self.SplineRef`)
    (:`Is Valid`
      (set `self.SplineDelta` 0.0)
      (set `self.Enabled` true)
      (`SceneComponent.SetHiddenInGame` _capsulecomponent false true)
      (`PrimitiveComponent.SetCollisionEnabled` _capsulecomponent "QueryAndPhysics"))
    (:`Is Not Valid`
      (`KismetSystemLibrary.PrintString` "No Valid Spline"))))

(fn `GetSplineLocRot`
  (params (Spline :type "SplineComponent Object Reference") (Distance :type "Float (double-precision)"))
  (returns (ReturnValue :type "Vector Structure") (ReturnValue2 :type "Rotator Structure"))
  (return (`SplineComponent.GetLocationAtDistanceAlongSpline` Spline Distance "World") (`SplineComponent.GetRotationAtDistanceAlongSpline` Spline Distance "World")))

(fn `Set Variables`
  (params (Spline :type "/Game/Systems/Level/SplineFollow/BP_SimpleSplineFollow Object Reference") (Speed :type "Float (double-precision)") (`Auto Activate` :type Boolean))
  (set `self.SplineRef` Spline)
  (set `self.Speed` Speed)
  (set `self.AutoActivate` `Auto Activate`))

(fn `UserConstructionScript`)