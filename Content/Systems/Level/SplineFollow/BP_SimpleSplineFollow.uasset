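; Simple spline-follow actor that drives one of two child-actor followers, a monster or another object, chosen by the Monster flag.
; The Construction Script casts the selected child actor and passes it this actor as Spline, along with Speed and AutoActivate.
; The StartSpline event calls FollowSpline on that same child, leaving the movement logic to the child Blueprint.
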(event `self.ReceiveBeginPlay`)

(event `StartSpline`
  (if (`self.Monster?`)
    (bind _asbp_monster_spline_follow (cast `/Game/Systems/Level/SplineFollow/BP_MonsterSplineObject` (`ChildActorComponent.ChildActor` (`self.BP_FollowSplineObject`))))
    (`/Game/Systems/Level/SplineFollow/BP_MonsterSplineObject.FollowSpline` _asbp_monster_spline_follow)
    (else
      (bind _asbp_other_spline_follow (cast `/Game/Systems/Level/SplineFollow/BP_OtherSplineObject` (`ChildActorComponent.ChildActor` (`self.BP_OtherSplineFollow`))))
      (`/Game/Systems/Level/SplineFollow/BP_OtherSplineObject.FollowSpline` _asbp_other_spline_follow))))

(fn `UserConstructionScript`
  (bind _speed (`self.Speed`))
  (bind _auto_activate (`self.Auto Activate`))
  (if (`self.Monster?`)
    (bind _asbp_monster_spline_follow (cast `/Game/Systems/Level/SplineFollow/BP_MonsterSplineObject` (`ChildActorComponent.ChildActor` (`self.BP_FollowSplineObject`))))
    (`/Game/Systems/Level/SplineFollow/BP_MonsterSplineObject.Set Variables` _asbp_monster_spline_follow self _speed _auto_activate)
    (else
      (bind _asbp_other_spline_follow (cast `/Game/Systems/Level/SplineFollow/BP_OtherSplineObject` (`ChildActorComponent.ChildActor` (`self.BP_OtherSplineFollow`))))
      (`/Game/Systems/Level/SplineFollow/BP_OtherSplineObject.Set Variables` _asbp_other_spline_follow self _speed _auto_activate))))