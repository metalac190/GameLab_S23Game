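; BP_GlassWithAnchor is a breakable glass actor that shatters on an optional trigger-box overlap or a debug NumPad 0 press.
; Construction registers four child anchor fields as initialization fields on the glass Geometry Collection.
; Shattering hides the intact glass, disables its and the trigger's collision, and reveals the simulated pieces.
; A once-only step then fires a child master field with configurable torque, force and falloff, and plays a random sound.
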(event `Glass Shatter`
  ;[1 1 1] Applying variables and triggering the MasterField (Forces)
  (add `self.GlassShatterEventDispatcher` (delegate `Glass Shatter`))
  (`self.SmashGlass` (`self.Glass`))
  (`/Engine/EditorBlueprintResources/StandardMacros.DoOnce` false
    (:`Completed`
      (bind _asfs_custom_master_field (cast `/Game/Systems/Level/Breakable/FS_CustomMasterField` (`ChildActorComponent.ChildActor` (`self.FS_CustomMasterField`))))
      (set `/Game/Systems/Level/Breakable/FS_CustomMasterField.TorqueMult` (`self.TorqueMult`) _asfs_custom_master_field)
      (set `/Game/Systems/Level/Breakable/FS_CustomMasterField.DirectionalMagnitude` (`self.Directional Force`) _asfs_custom_master_field)
      (if (`self.VelocityFalloff`)
        (set `/Game/Systems/Level/Breakable/FS_CustomMasterField.VelocityFieldFalloffType` "Field_Falloff_Linear" _asfs_custom_master_field)
        (else
          (set `/Game/Systems/Level/Breakable/FS_CustomMasterField.VelocityFieldFalloffType` "Field_FallOff_None" _asfs_custom_master_field)))
      (`/Game/Systems/Level/Breakable/FS_CustomMasterField.CE_Trigger` _asfs_custom_master_field)
      (`GameplayStatics.PlaySoundAtLocation` (`KismetArrayLibrary.Array_Random` (`self.SoundArray`)) (`SceneComponent.K2_GetComponentLocation` (`self.DefaultSceneRoot`)) (struct) 1.0 1.0 0.0 null null null null))))

(event `self.Box.OnComponentBeginOverlap`
  (params (OverlappedComponent :type "PrimitiveComponent Object Reference") (OtherActor :type "Actor Object Reference") (OtherComp :type "PrimitiveComponent Object Reference") (OtherBodyIndex :type Integer) (bFromSweep :type Boolean) (SweepResult :type "HitResult Structure (by ref)"))
  ;[1 1 1] Trigger Box
  (if (`self.UsesCollisionTrigger`)
    (`self.Glass Shatter`)))

(event `self.ReceiveBeginPlay`
  ;[1 1 1] Debug
  (`self.EnableInput` (`GameplayStatics.GetPlayerController` 0)))

(event `Key|NumPadZero`
  (params (Key :type "Key Structure"))
  ;[1 1 1] Debug
  (:`Pressed`
    (`self.Glass Shatter`)))

(fn `SmashGlass`
  (params (Glass :type "StaticMeshComponent Object Reference"))
  (bind _glass_geometrycollection (`self.Glass_GeometryCollection`))
  ;[1 1 1] Swapping Glass with Broken Pieces
  (`/Engine/EditorBlueprintResources/StandardMacros.IsValid` Glass
    (:`Is Valid`
      (if (not (`ActorComponent.IsBeingDestroyed` Glass))
        (`PrimitiveComponent.SetCollisionEnabled` Glass "NoCollision")
        (`PrimitiveComponent.SetCollisionEnabled` (`self.Box`) "NoCollision")
        (`PrimitiveComponent.SetSimulatePhysics` _glass_geometrycollection true)
        (`SceneComponent.SetHiddenInGame` _glass_geometrycollection false false)
        (`SceneComponent.SetHiddenInGame` Glass true false)))))

(fn `UserConstructionScript`
  ;[1 1 1] Anchor Setup
  (for _array_element (`|MakeArray` (`ChildActorComponent.ChildActor` (`self.FS_CustomAnchorField`)) (`ChildActorComponent.ChildActor` (`self.FS_CustomAnchorField1`)) (`ChildActorComponent.ChildActor` (`self.FS_CustomAnchorField2`)) (`ChildActorComponent.ChildActor` (`self.FS_CustomAnchorField3`)))
    (bind _asfs_custom_anchor_field (cast `/Game/Systems/Level/Breakable/FS_CustomAnchorField` _array_element))
    (`KismetArrayLibrary.Array_Add` (`GeometryCollectionComponent.InitializationFields` (`self.Glass_GeometryCollection`)) _asfs_custom_anchor_field)))