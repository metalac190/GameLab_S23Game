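; BP_TestBranch is a breakable Geometry Collection branch that shatters once when the player overlaps it, unless their capsule half height shows a specific lowered value, likely crouching.
; Construction registers a child-actor anchor field as an initialization field and picks a random rest collection.
; On overlap, it passes torque and radial force to a child-actor master field, triggers it, plays a random sound and reports noise, presumably for AI hearing.
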(event `self.Box.OnComponentBeginOverlap`
  (params (OverlappedComponent :type "PrimitiveComponent Object Reference") (OtherActor :type "Actor Object Reference") (OtherComp :type "PrimitiveComponent Object Reference") (OtherBodyIndex :type Integer) (bFromSweep :type Boolean) (SweepResult :type "HitResult Structure (by ref)"))
  (bind _returnvalue (`SceneComponent.K2_GetComponentLocation` (`self.DefaultSceneRoot`)))
  (bind _asbp_player (cast `/Game/Entities/Player/BP_Player` OtherActor))
  (if (not (== (`CapsuleComponent.GetScaledCapsuleHalfHeight` (`Character.CapsuleComponent` _asbp_player)) 45.0))
    (`/Engine/EditorBlueprintResources/StandardMacros.DoOnce` false
      (:`Completed`
        (bind _asfs_custom_master_field (cast `/Game/Systems/Level/Breakable/FS_CustomMasterField` (`ChildActorComponent.ChildActor` (`self.FS_CustomMasterField`))))
        (set `/Game/Systems/Level/Breakable/FS_CustomMasterField.TorqueMult` (`self.TorqueMult`) _asfs_custom_master_field)
        (set `/Game/Systems/Level/Breakable/FS_CustomMasterField.Radial Magnitude` (`self.RadialForce`) _asfs_custom_master_field)
        (`/Game/Systems/Level/Breakable/FS_CustomMasterField.CE_Trigger` _asfs_custom_master_field)
        (`GameplayStatics.PlaySoundAtLocation` (`KismetArrayLibrary.Array_Random` (`self.SoundArray`)) _returnvalue (struct) 1.0 1.0 0.0 null null null null)
        (`AISense_Hearing.ReportNoiseEvent` _returnvalue 1.0 self)))))

(fn `UserConstructionScript`
  (`|ExecutionSequence`
    (:`then_0`
      (bind _asfs_custom_anchor_field (cast `/Game/Systems/Level/Breakable/FS_CustomAnchorField` (`ChildActorComponent.ChildActor` (`self.FS_CustomAnchorField`))))
      (`KismetArrayLibrary.Array_Add` (`GeometryCollectionComponent.InitializationFields` (`self.TestBranch_GeometryCollection`)) _asfs_custom_anchor_field))
    (:`then_1`
      (`GeometryCollectionComponent.SetRestCollection` (`self.TestBranch_GeometryCollection`) (`KismetArrayLibrary.Array_Random` (`self.MeshArray`))))))