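; Player component that tracks a collectible storybook: which pages have been found and which spread is open.
; On BeginPlay it builds a map of page name, image and number from data table rows.
; AddPage records found pages, while the flip events move the current page by two within the book's bounds.
; GetPageInfo looks up a page by index, substituting a 404 placeholder image for any page not yet found.
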(event `self.ReceiveBeginPlay`
  (bind _outrownames (`DataTableFunctionLibrary.GetDataTableRowNames` (`self.DTStorybook`)))
  (set `self.storybookLength` (`KismetArrayLibrary.Array_Length` _outrownames))
  (for (_array_element _array_index) _outrownames
    (bind _returnvalue (`|GetDataTableRow` "/Game/Data/StorybookPages.StorybookPages" _array_element)
      (:`then`
        (`BlueprintMapLibrary.Map_Add` (`self.pageInfoMap`) _array_element (make `/Game/Systems/Structures/Storybook/PageInfo` _array_element (`.Image_3_7B6234204F03C062D2C19992E7992FD0` (break `/Game/Systems/Structures/Storybook/PageImage` _returnvalue)) (+ _array_index 1)))))))

(event `Add Page`
  (params (`Page Name` :type Name))
  (`BlueprintSetLibrary.Set_Add` (`self.pagesFound`) `Page Name`))

(event `Flip Page Left`
  (if (not (== (`self.current page`) 0))
    (set `self.current page` (- (`self.current page`) 2))))

(event `Flip Page Right`
  (if (< (`self.current page`) (- (`self.storybookLength`) 2))
    (set `self.current page` (+ (`self.current page`) 2))))

(fn `Get_Page_Info`
  (params (index :type Integer))
  (returns (PageInfo :type "/Game/Systems/Structures/Storybook/PageInfo Structure"))
  (locals (Image :type "Texture2D Object Reference"))
  (bind _pageinfomap (`self.pageInfoMap`))
  (bind _keys (`BlueprintMapLibrary.Map_Keys` _pageinfomap))
  (bind _value (`BlueprintMapLibrary.Map_Find` _pageinfomap (`|GetArrayItem` _keys index)))
  (if (not (`BlueprintSetLibrary.Set_Contains` (`self.pagesFound`) (break `/Game/Systems/Structures/Storybook/PageInfo` _value)))
    (set `local.Image` "/Game/Art/StorybookPages/404Page.404Page")
    (else
      (set `local.Image` (`.Image_13_AF2B684340CCA38086B91596DD7403E0` (break `/Game/Systems/Structures/Storybook/PageInfo` _value)))))
  (return (make `/Game/Systems/Structures/Storybook/PageInfo` (break `/Game/Systems/Structures/Storybook/PageInfo` _value) (`local.Image`) (`.PageNumber_12_4B6AB89142DF46561D6F178EA88DBB30` (break `/Game/Systems/Structures/Storybook/PageInfo` _value)))))