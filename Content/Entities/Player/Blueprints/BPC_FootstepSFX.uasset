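; Actor component that plays surface-based footstep sounds while its owner moves along the ground.
; Tick checks horizontal velocity against a threshold with zero vertical speed, using a DoOnce to start a looping timer and clearing it when movement stops.
; Each timer step traces down from the owner and plays a wood, dirt or grass sound at the hit point by physical surface type, also printing debug text.
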(event `self.ReceiveTick`
  (params (DeltaSeconds :type "Float (single-precision)"))
  (bind _velocitythreshold (`self.VelocityThreshold`))
  (bind (_returnvalue_x _returnvalue_y _returnvalue_z) (`KismetMathLibrary.BreakVector` (`Actor.GetVelocity` (`self.GetOwner`))))
  (bind _returnvalue (* _velocitythreshold -1.0))
  (if (and (or (> _returnvalue_x _velocitythreshold) (< _returnvalue_x _returnvalue) (> _returnvalue_y _velocitythreshold) (< _returnvalue_y _returnvalue)) (== _returnvalue_z 0.0))
    (`/Engine/EditorBlueprintResources/StandardMacros.DoOnce` false :!label _label
      (:`Completed`
        (bind _returnvalue_2 (`KismetSystemLibrary.K2_SetTimerDelegate` (delegate `PlayFootstepSound`) (`self.FootstepInterval`) true))))
    (else
      (`KismetSystemLibrary.K2_ClearAndInvalidateTimerHandle` _returnvalue_2)
      (goto _label :!via `Reset`))))

(event `PlayFootstepSound`
  (bind _returnvalue (`Actor.K2_GetActorLocation` (`self.GetOwner`)))
  (bind _outhit (`KismetSystemLibrary.LineTraceSingle` _returnvalue (- _returnvalue (0.0 0.0 100.0)) "TraceTypeQuery1"))
  (switch `EPhysicalSurface` (`GameplayStatics.GetSurfaceType` _outhit)
    (:`SurfaceType1`
      (bind (_bblockinghit _binitialoverlap _time _distance _location) (`GameplayStatics.BreakHitResult` _outhit))
      (`GameplayStatics.PlaySoundAtLocation` "/Game/Audio/Footsteps/WoodFootstep.WoodFootstep" _location (struct) 1.0 1.0 0.0 null null null null)
      (`KismetSystemLibrary.PrintString` "Play Wood Footstep Sound"))
    (:`SurfaceType2`
      (`GameplayStatics.PlaySoundAtLocation` "/Game/Audio/Footsteps/DirtFootstep.DirtFootstep" _location (struct) 1.0 1.0 0.0 null null null null)
      (`KismetSystemLibrary.PrintString` "Play Dirt Footstep Sound"))
    (:`SurfaceType3`
      (`GameplayStatics.PlaySoundAtLocation` "/Game/Audio/Footsteps/GrassFootstep.GrassFootstep" _location (struct) 1.0 1.0 0.0 null null null null)
      (`KismetSystemLibrary.PrintString` "Play Grass Footstep Sound"))))