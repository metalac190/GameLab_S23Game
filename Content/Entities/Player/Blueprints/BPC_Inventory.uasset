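; Player inventory component that stores items in a fixed four-slot array.
; Adding an item forwards it to the player's crafter component when the crafter is equipped; otherwise it fills the first empty slot and updates the inventory widget, or returns false when full.
; An empty item name marks a free slot for lookups and adds, and removal blanks the matching slot without updating the UI.
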(event `self.ReceiveBeginPlay`
  (set `self.Inventory` (`|MakeArray` (struct) (struct) (struct) (struct) :!type "/Game/Entities/Gameplay/Items/S_ItemData Structure")))

(fn `AddToInventory`
  (params (NewItem :type "/Game/Entities/Gameplay/Items/S_ItemData Structure (by ref)"))
  (returns (ItemAdded :type Boolean))
  (bind _inventory (`self.Inventory`))
  ;[1 1 1] Add to crafter if equipped
  (bind _asbp_player (cast `/Game/Entities/Player/Blueprints/BP_Player` (`self.GetOwner`)))
  (if (`/Game/Entities/Player/Blueprints/BP_Player.crafterEquipped` _asbp_player)
    (`/Game/Systems/Mechanics/Crafting/BPC_Crafter.Add Item` (`/Game/Entities/Player/Blueprints/BP_Player.BPC_Crafter` _asbp_player) NewItem)
    (return true)
    (else
      (for (_array_element _array_index) _inventory
        (if (`KismetStringLibrary.IsEmpty` (break `/Game/Entities/Gameplay/Items/S_ItemData` _array_element))
          (break)
          (elif (== _array_index (- (`KismetArrayLibrary.Array_Length` _inventory) 1))
            (return false))))
      (bind _output_get (set `self.FirstEmptySlotIndex` _array_index))
      (`|VariableSetRef` (`|GetArrayItem` _inventory _output_get) NewItem) ; set first empty inventory index to new item
      (bind _asbp_player_2 (cast `/Game/Entities/Player/Blueprints/BP_Player` (`self.GetOwner`))
        (:`then`
          (`/Game/UI/Widgets/WB_InventoryWidget.AddItemToUI` (`/Game/Entities/Player/Blueprints/BP_Player.InventoryWidget` _asbp_player_2) (`.ItemName_18_CD23B635439CECA1569C62A2D3CDE386` (break `/Game/Entities/Gameplay/Items/S_ItemData` NewItem)) (`self.FirstEmptySlotIndex`)) ; adds the item to the inventory UI\nTODO: display the image, not the name
          (return true))
        (:`CastFailed`
          (`KismetSystemLibrary.PrintText` "Cast to BP_Player failed"))))))

(fn `GetStoredItem`
  (params (ItemIndex :type Integer))
  (returns (ItemFound :type Boolean) (StoredItem :type "/Game/Entities/Gameplay/Items/S_ItemData Structure"))
  (bind _output (`|GetArrayItem` (`self.Inventory`) ItemIndex))
  (if (not (`KismetStringLibrary.IsEmpty` (`.ItemName_18_CD23B635439CECA1569C62A2D3CDE386` (break `/Game/Entities/Gameplay/Items/S_ItemData` _output))))
    (return true _output)
    (else
      (return false))))

(fn `RemoveFromInventory`
  (params (ItemToRemove :type "/Game/Entities/Gameplay/Items/S_ItemData Structure"))
  (bind _inventory (`self.Inventory`))
  (`KismetArrayLibrary.Array_Set` _inventory (`KismetArrayLibrary.Array_Find` _inventory ItemToRemove)) ; set the inventory slot with\nthe item to empty
)