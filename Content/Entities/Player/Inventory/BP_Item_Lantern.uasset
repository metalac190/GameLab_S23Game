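; BP_Item_Lantern is a lantern item among the player's inventory assets, with a Cone component hung by a physics constraint and a cable.
; Both the construction script and BeginPlay set the Cone as the constraint's second component and attach the cable's end to it, after calling the parent.
; GetItemData returns without supplying any values, and the Tick and overlap events are unused.
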(event `self.ReceiveBeginPlay`
  (`parent.ReceiveBeginPlay`)
  (`PhysicsConstraintComponent.SetConstrainedComponents` (`self.PhysicsConstraint`) null "None" (`self.Cone`) "None")
  (`CableComponent.SetAttachEndToComponent` (`self.Cable`) (`self.Cone`) "None"))

(fn `GetItemData`
  (returns (ItemData :type "/Game/Entities/Player/Inventory/S_ItemData Structure"))
  (return))

(fn `UserConstructionScript`
  (`parent.UserConstructionScript`)
  (`PhysicsConstraintComponent.SetConstrainedComponents` (`self.PhysicsConstraint`) null "None" (`self.Cone`) "None")
  (`CableComponent.SetAttachEndToComponent` (`self.Cable`) (`self.Cone`) "None"))