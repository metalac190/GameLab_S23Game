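; Art actor that builds tapering roots along an editable spline.
; The construction script adds a Z-forward spline mesh for each segment between spline points, using the assigned mesh and optional physics-only collision.
; GetTaperedScale sets each segment's end scales from normalized spline distance, ramping from full thickness at TaperStart to TaperScale at the tip.
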(fn `GetTaperedScale`
  (params (Spline :type "SplineComponent Object Reference") (SplineIndex :type Integer))
  (returns (Ratio :type "Vector2D Structure"))
  (bind _returnvalue (* (`KismetMathLibrary.MapRangeClamped` (`KismetMathLibrary.SafeDivide` (`SplineComponent.GetDistanceAlongSplineAtSplinePoint` Spline SplineIndex) (`SplineComponent.GetSplineLength` Spline)) (`self.TaperStart`) 1.0 1.0 (`self.TaperScale`)) (`self.Thickness`)))
  (return (`KismetMathLibrary.MakeVector2D` _returnvalue _returnvalue)))

(fn `UserConstructionScript`
  (locals (SplineMeshComponent :type "SplineMeshComponent Object Reference") (SplineIndexStart :type Integer) (SplineIndexEnd :type Integer))
  (bind _splineindexstart (`local.SplineIndexStart`))
  (bind _spline (`self.Spline`))
  (bind _splineindexend (`local.SplineIndexEnd`))
  (bind _splinemeshcomponent (`local.SplineMeshComponent`))
  (for _index (range (+ (- (`SplineComponent.GetNumberOfSplinePoints` (`self.Spline`)) 2) 1))
    (set `local.SplineIndexStart` _index)
    (set `local.SplineIndexEnd` (+ _index 1))
    (bind _returnvalue (`AddComponent|NODE_AddSplineMeshComponent-0`))
    (bind _output_get (set `local.SplineMeshComponent` _returnvalue))
    (`SplineMeshComponent.SetForwardAxis` _output_get "Z" true)
    (`StaticMeshComponent.SetStaticMesh` (`local.SplineMeshComponent`) (`self.Mesh`))
    (`SceneComponent.K2_AttachToComponent` (`local.SplineMeshComponent`) (`self.DefaultSceneRoot`) "None" "KeepRelative" "KeepRelative" "KeepRelative" true)
    (`SplineMeshComponent.SetStartAndEnd` (`local.SplineMeshComponent`) (`SplineComponent.GetLocationAtSplinePoint` _spline _splineindexstart "Local") (`SplineComponent.GetTangentAtSplinePoint` _spline _splineindexstart "Local") (`SplineComponent.GetLocationAtSplinePoint` _spline _splineindexend "Local") (`SplineComponent.GetTangentAtSplinePoint` _spline _splineindexend "Local") true)
    (bind _ratio (`self.GetTaperedScale` (`self.Spline`) (`local.SplineIndexStart`)))
    (`SplineMeshComponent.SetStartScale` (`local.SplineMeshComponent`) _ratio true)
    (bind _ratio_2 (`self.GetTaperedScale` (`self.Spline`) (`local.SplineIndexEnd`)))
    (`SplineMeshComponent.SetEndScale` (`local.SplineMeshComponent`) _ratio_2 true)
    (if (`self.EnableCollisions`)
      (`PrimitiveComponent.SetCollisionEnabled` _splinemeshcomponent "PhysicsOnly")
      (else
        (`PrimitiveComponent.SetCollisionEnabled` _splinemeshcomponent "NoCollision")))))