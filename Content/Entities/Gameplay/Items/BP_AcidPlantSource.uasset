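; BP_AcidPlantSource is an interactable acid plant that the player tries to collect into a bucket.
; Interact locks re-entry, checks CanUse and plays a success or fail montage on the first-person hands, blanking the prompt meanwhile.
; Montage notifies time the effects: success hides the plant mesh on touch and calls parent Interact on bucket placement.
; Failure plays the plant's own fail montage on touch and re-enables interaction on completion.
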(event `/Game/Systems/Mechanics/BP_InteractableInterface.Interact`
  (params (Player :type "/Game/Entities/Player/BP_Player Object Reference"))
  (bind _firstperson_hands (`/Game/Entities/Player/BP_Player.FirstPerson_Hands` Player))
  (if (`self.bCanInteract`)
    (set `self.bCanInteract` false)
    (bind _returnvalue (`self.Can Use` Player))
    (if _returnvalue
      (bind _notifyname (`|PlayMontage` _firstperson_hands "/Game/Art/_Global/First_Person_Hands/Anim/Bucket_Plant_Interact_Success_Montage.Bucket_Plant_Interact_Success_Montage")
        (:`then`
          (`/Game/Entities/Player/BP_Player.SetPromptForDuration` Player null " " 10.0 :!label _label))
        (:`OnCompleted`
          (`/Game/Entities/Player/BP_Player.SetPromptForDuration` Player null " " 0.0 :!label _label_2))
        (:`OnNotifyBegin`
          (switch `name` _notifyname
            (:`Touch`
              (`SceneComponent.SetVisibility` (`self.SkeletalMesh`) false false))
            (:`PlaceInBucket`
              (`parent.Interact` Player)))))
      (else
        (bind _notifyname_2 (`|PlayMontage` _firstperson_hands "/Game/Art/_Global/First_Person_Hands/Anim/Bucket_Plant_Interact_Fail_Montage.Bucket_Plant_Interact_Fail_Montage")
          (:`then`
            (goto _label))
          (:`OnCompleted`
            (set `self.bCanInteract` true)
            (goto _label_2))
          (:`OnNotifyBegin`
            (switch `name` _notifyname_2
              (:`Touch`
                (`AnimInstance.Montage_Play` (`SkeletalMeshComponent.GetAnimInstance` (`self.SkeletalMesh`)) "/Game/Art/01_Basement/acidPlant/Anim/SM_acidPlant_root_Interaction_Fail_Montage.SM_acidPlant_root_Interaction_Fail_Montage" 1.0 "MontageLength" 0.0 true)))))))))

(fn `UserConstructionScript`
  (`parent.UserConstructionScript`))