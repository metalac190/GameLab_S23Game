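; BP_ItemSource is an interactable pickup that gives its configured item to the player's inventory once.
; On BeginPlay it caches the item's data, then Interact plays a clink sound and adds it through BPCInventory, setting ItemInUse to block repeat grabs.
; An optional flag restricts interaction to players with the crafter equipped.
; GetPrompt mirrors these conditions, showing the action with item name, an already-grabbed message or a missing-tool hint.
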(event `self.ReceiveBeginPlay`
  (bind _itemdata (`/Game/Systems/Utility/ItemMacroLibrary.GetItemData` (`self.Item`))
    (:`OutExec`
      (set `self.ItemData` _itemdata))))

(event `/Game/Systems/Mechanics/BP_InteractableInterface.Interact`
  (params (Player :type "/Game/Entities/Player/BP_Player Object Reference"))
  (if (or (`/Game/Entities/Player/BP_Player.crafterEquipped` Player) (not (`self.onlyUseWhenCrafterEquipped`)))
    (`GameplayStatics.PlaySound2D` "/Game/Audio/Gameplay/Scratch/sfx_item_bottleClink_0.sfx_item_bottleClink_0" 1.0 1.0 0.0 null null)
    (if (`self.ItemInUse`)
      (`KismetSystemLibrary.PrintString` "Alreadying Gradbbed this item")
      (else
        (set `self.ItemInUse` true)
        (`/Game/Systems/Player/BPC_Inventory.AddToInventory` (`/Game/Entities/Player/BP_Player.BPC_Inventory` Player) (`self.ItemData`))))))

(fn `GetPrompt`
  (params (player :type "/Game/Entities/Player/BP_Player Object Reference"))
  (returns (inputAction :type "InputAction Object Reference") (actionText :type Text))
  (bind _itemdata_itemname (break `/Game/Entities/Gameplay/Items/S_ItemData` (`self.ItemData`)))
  (if (`self.ItemInUse`)
    (return null "already grabbed this item")
    (elif (or (`/Game/Entities/Player/BP_Player.crafterEquipped` player) (not (`self.onlyUseWhenCrafterEquipped`)))
      (return "/Game/Entities/Player/Input/IA_Interact.IA_Interact" (`KismetTextLibrary.Conv_StringToText` (`KismetStringLibrary.Concat_StrStr` (`self.actionText`) " " _itemdata_itemname)))
      (else
        (return null "You need something to use this with")))))

(fn `UserConstructionScript`)