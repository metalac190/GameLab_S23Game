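; BP_ITEM_MASTER is the master pickup item actor, holding item data and a static mesh for world interaction.
; BeginPlay copies the mesh into ItemData, while SetData applies incoming data to the mesh or destroys the actor when the name is empty.
; Interact adds the item to the player's inventory component, then equips it, notifies pickup and destroys the actor, or prints an inventory-full message.
; GetPrompt supplies the interact input and item-name text.
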(event `self.ReceiveBeginPlay`
  (setmembers `/Game/Entities/Gameplay/Items/S_ItemData` :`StructRef` (`self.ItemData`) :`ItemMesh` (`StaticMeshComponent.StaticMesh` (`self.StaticMesh`))))

(event `/Game/Systems/Mechanics/BP_InteractableInterface.Interact`
  (params (Player :type "/Game/Entities/Player/BP_Player Object Reference"))
  (bind _itemdata (`self.Get Item Data`))
  (bind (_itemadded _index) (`/Game/Systems/Player/BPC_Inventory.AddToInventory` (`/Game/Entities/Player/BP_Player.BPC_Inventory` Player) _itemdata))
  (if _itemadded
    (`/Game/Entities/Player/BP_Player.EquipItem` Player _index)
    (`/Game/Entities/Player/BP_Player.ItemPickedUp` Player _itemdata)
    (`self.K2_DestroyActor`)
    (else
      (`KismetSystemLibrary.PrintString` "Could not add item. Inventory is full."))))

(fn `Get Item Data`
  (returns (ItemData :type "/Game/Entities/Gameplay/Items/S_ItemData Structure"))
  (return (`self.ItemData`)))

(fn `GetPrompt`
  (params (player :type "/Game/Entities/Player/BP_Player Object Reference"))
  (returns (inputAction :type "InputAction Object Reference") (actionText :type Text))
  (bind _itemdata_itemname (break `/Game/Entities/Gameplay/Items/S_ItemData` (`self.ItemData`)))
  (return "/Game/Entities/Player/Input/IA_Interact.IA_Interact" (`KismetTextLibrary.Conv_StringToText` (`KismetStringLibrary.Concat_StrStr` (`self.actionText`) " " _itemdata_itemname))))

(fn `Set Data`
  (params (InputData :type "/Game/Entities/Gameplay/Items/S_ItemData Structure"))
  (returns (DestroyedItem :type Boolean))
  (bind _output_get (set `self.ItemData` InputData))
  (if (`KismetStringLibrary.IsEmpty` (break `/Game/Entities/Gameplay/Items/S_ItemData` _output_get))
    (`self.K2_DestroyActor`)
    (return true)
    (else
      (`StaticMeshComponent.SetStaticMesh` (`self.StaticMesh`) (`.ItemMesh_12_7EE7D8D84E9FEE43260F5A97623E8EBD` (break `/Game/Entities/Gameplay/Items/S_ItemData` _output_get)))
      (return false))))

(fn `UserConstructionScript`)