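; BP_ItemLantern is a lantern item that switches between regular fire and blue magic fire.
; ActivateLantern flips IsOn, setting the state to Normal when on and Magic when off, so toggling off shows magic fire rather than extinguishing it.
; Tick reapplies the sphere material and both fire components' active flags from the state every frame.
; An Empty state with a solid material is handled but never set here.
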(event `self.ReceiveBeginPlay`
  (`parent.ReceiveBeginPlay`))

(event `ActivateLantern`
  (if (`self.isOn`)
    (set `self.isOn` false)
    (else
      (set `self.isOn` true)))
  (if (`self.isOn`)
    (set `self.CurrentState` "Normal")
    (else
      (set `self.CurrentState` "Magic"))))

(event `self.ReceiveTick`
  (params (DeltaSeconds :type "Float (single-precision)"))
  (bind _sphere (`self.Sphere`))
  (switch `string` (`self.CurrentState`)
    (:`Normal`
      ;[1 1 1] Change behavior based on state
      (`PrimitiveComponent.SetMaterial` _sphere 0 "/Game/Levels/LevelPrototyping/Materials/M_Glow.M_Glow")
      (`ActorComponent.SetActive` (`self.RegularFire`) (`self.isOn`) false :!label _label)
      (`ActorComponent.SetActive` (`self.MagicFire`) false false))
    (:`Empty`
      (`PrimitiveComponent.SetMaterial` _sphere 0 "/Game/Levels/LevelPrototyping/Materials/M_Solid.M_Solid")
      (goto _label))
    (:`Magic`
      (`PrimitiveComponent.SetMaterial` _sphere 0 "/Game/Levels/LevelPrototyping/Materials/MI_Solid_Blue.MI_Solid_Blue")
      (`ActorComponent.SetActive` (`self.RegularFire`) false false)
      (`ActorComponent.SetActive` (`self.MagicFire`) true false))))

(fn `UserConstructionScript`
  (`parent.UserConstructionScript`))