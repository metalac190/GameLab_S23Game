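; BP_PageObject is an interactable collectible page that is added to the player's storybook and then destroyed.
; Pickup requires the page to be enabled and the player's BPCStorybook to have a book; GetPrompt reflects both conditions.
; The construction script hides disabled pages, and FadeIn enables and reveals one, using a timeline to animate its scale.
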(event `/Game/Systems/Mechanics/BP_InteractableInterface.Interact`
  (params (Player :type "/Game/Entities/Player/BP_Player Object Reference"))
  (bind _bpc_storybook (`/Game/Entities/Player/BP_Player.BPC_Storybook` Player))
  (bind _page_name (`self.Page Name`))
  (if (`self.Enabled`)
    (if (`/Game/Systems/Mechanics/Storybook/BPC_Storybook.hasBook` _bpc_storybook)
      (`/Game/Systems/Mechanics/Storybook/BPC_Storybook.Add Page` _bpc_storybook _page_name)
      (`/Game/Entities/Player/BP_Player.PagePickedUp` Player _page_name)
      (`self.K2_DestroyActor`))))

(event `Fade In`
  (bind (_returnvalue_location _returnvalue_rotation _returnvalue_scale) (`KismetMathLibrary.BreakTransform` (`SceneComponent.GetRelativeTransform` (`self.Scene`))))
  (set `self.Enabled` true)
  (`self.SetActorHiddenInGame` false)
  (set `self.finalScale` _returnvalue_scale)
  (bind (_direction _scale) (`Timeline|FadeInTimeline`)
    (:`Update`
      (`SceneComponent.SetWorldScale3D` (`self.Scene`) (* (`KismetMathLibrary.Conv_DoubleToVector` _scale) (`self.finalScale`))))))

(event `self.ReceiveBeginPlay`)

(fn `GetPrompt`
  (params (player :type "/Game/Entities/Player/BP_Player Object Reference"))
  (returns (inputAction :type "InputAction Object Reference") (actionText :type Text))
  (if (`self.Enabled`)
    (if (`/Game/Systems/Mechanics/Storybook/BPC_Storybook.hasBook` (`/Game/Entities/Player/BP_Player.BPC_Storybook` player))
      (return "/Game/Entities/Player/Input/IA_Interact.IA_Interact" "collect page")
      (else
        (return null "you need something to use this with")))
    (else
      (return null ""))))

(fn `UserConstructionScript`
  (`self.SetActorHiddenInGame` (not (`self.Enabled`))))