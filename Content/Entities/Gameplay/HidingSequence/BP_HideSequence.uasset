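; BP_HideSequence runs a timed hiding challenge in which the player must get into one of its valid hiding volumes.
; Tick detects early hiding during the countdown; otherwise a final check on timeout decides success or failure, reported through dispatchers.
; Once successfully hidden, leaving cover triggers camera shake, failure and sequence end.
; Helper functions expose the occupied volume's monster destination and spline path, with player location as the destination fallback.
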(event `self.ReceiveBeginPlay`
  (if (`self.AutoStartHideSequence`)
    (`self.StartHideSequence`)
    (bind _asbp_player (cast `/Game/Entities/Player/BP_Player` (`GameplayStatics.GetPlayerCharacter` 0)))
    (set `self.Player` _asbp_player)))

(event `StartHideSequence`
  (`KismetSystemLibrary.PrintString` "HIDE START")
  (set `self.HidBeforeDelay` false)
  (set `self.SequenceDelayCompleted` false)
  (set `self.HideSequenceStarted` true)
  (`KismetSystemLibrary.RetriggerableDelay` (`self.SequenceLength`))
  (`KismetSystemLibrary.PrintString` "HIDE STOP")
  (set `self.SequenceDelayCompleted` true)
  (if (not (`self.HidBeforeDelay`))
    (`self.CheckPlayerHidden`)
    (if (`self.PlayerHidden`)
      (`self.PlayerSuccessfullyHidden`)
      (set `self.ActivelyHiding` true)
      (else
        (`self.PlayerNotHidden`)
        (`KismetSystemLibrary.PrintString` "this level sucks")))))

(event `self.ReceiveTick`
  (params (DeltaSeconds :type "Float (single-precision)"))
  (`|ExecutionSequence`
    (:`then_0`
      (if (`self.ActivelyHiding`)
        (`self.CheckPlayerHidden`)
        (if (not (`self.PlayerHidden`))
          (`/Game/Entities/Player/BP_Player.FeedbackMasterNode` (`self.Player`) true null null 0.0 0.0)
          (`self.PlayerNotHidden`)
          (`self.EndHideSequence`))))
    (:`then_1`
      (if (`self.HideSequenceStarted`)
        (if (`self.SequenceDelayCompleted`)
          _
          (elif (not (`self.HidBeforeDelay`))
            (`self.CheckPlayerHidden`)
            (if (`self.PlayerHidden`)
              (`self.PlayerSuccessfullyHidden`)
              (`KismetSystemLibrary.PrintString` "THIS IS WORKINGGGGG :DDD")
              (set `self.ActivelyHiding` true)
              (set `self.HidBeforeDelay` true))))))))

(event `EndHideSequence`
  (set `self.ActivelyHiding` false)
  (`KismetSystemLibrary.PrintString` "End Hiding Sequence"))

(event `PlayerSuccessfullyHidden`
  ;[1 1 1] Event Dispatchers
  (`KismetSystemLibrary.PrintString` "Hidden Successfully, Notify Level Blueprint")
  (`self.PlayerHiddenSuccessfully`))

(event `PlayerNotHidden`
  ;[1 1 1] Event Dispatchers
  (`KismetSystemLibrary.PrintString` "You're Dead. But Wake up and keep playing.")
  (`self.PlayerFailedToHide`))

(fn `CheckPlayerHidden`
  (`|ExecutionSequence`
    (:`then_0`
      (set `self.PlayerHidden` false))
    (:`then_1`
      (for _array_element (`self.ValidVolumes`)
        (if (`/Game/Entities/Gameplay/HidingSequence/BP_HideVolume.PlayerHidden` _array_element)
          (set `self.PlayerHidden` true)
          (set `self.Volume Player Hide In` _array_element))))))

(fn `GetMonsterSplinePath`
  (returns (SplinePath :type "SplineComponent Object Reference"))
  (for _array_element (`self.ValidVolumes`)
    (if (`/Game/Entities/Gameplay/HidingSequence/BP_HideVolume.PlayerHidden` _array_element)
      (return (`/Game/Entities/Gameplay/HidingSequence/BP_HideVolume.Spline` _array_element))))
  (return null))

(fn `GetMonsterTravelTo`
  (returns (Location :type "Vector Structure"))
  (for _array_element (`self.ValidVolumes`)
    (if (`/Game/Entities/Gameplay/HidingSequence/BP_HideVolume.PlayerHidden` _array_element)
      (bind _monstertraveltoposition_location (`KismetMathLibrary.BreakTransform` (`/Game/Entities/Gameplay/HidingSequence/BP_HideVolume.MonsterTravelToPosition` _array_element)))
      (return _monstertraveltoposition_location)))
  (return (`self.K2_GetActorLocation` (`GameplayStatics.GetPlayerPawn` 0))))

(fn `UserConstructionScript`)