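; Moondial puzzle where the player places a lantern, then matching coins to unlock and advance moon phases.
; Tick moves CurrentPhase toward GoalPhase, blending moon rotation, directional and lantern lights, turning the ring and opening each phase's vine doors past halfway.
; Left/right input selects among unlocked phases, though backward steps snap without refreshing visuals.
; Reaching New Moon completes the dial, returns the lantern and fires a completion event.
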(event `self.ReceiveBeginPlay`
  (bind _fullmoon (`self.FullMoon`))
  ;[1 1 1] Begin Play
  (`SceneComponent.SetVisibility` (`self.LanternLight`) false false)
  (`self.HideAllPhaseCoins`)
  (bind _outactors (`GameplayStatics.GetAllActorsOfClass` "/Script/Engine.DirectionalLight"))
  (set `self.DirLight` (`|GetArrayItem` _outactors))
  (`self.SetPhase` _fullmoon _fullmoon)
  (set `self.GoalPhase` (`KismetMathLibrary.Conv_IntToDouble` (`self.StartPhase (Debug Only)`)))
  (`ActorComponent.SetActive` (`self.Moondial Camera`) false false)
  (set `self.CanInteract` true)
  (bind _asbp_player (cast `/Game/Entities/Player/BP_Player` (`GameplayStatics.GetPlayerPawn` 0)))
  (bind _output_get (set `self.Player` _asbp_player))
  (add `/Game/Entities/Player/BP_Player.OnItemEquipped` _output_get (delegate `CheckPlayerUseItem`)))

(event `CheckPlayerUseItem`
  (params (ItemName :type String))
  ;[1 1 1] Begin Play
  (if (`/Game/Entities/Player/BP_Player.MoondialLock` (stale `self.ReceiveBeginPlay` _output_get))
    (`/Game/Systems/Mechanics/BP_InteractableInterface.Interact` (stale `self.ReceiveBeginPlay` _output_get))))

(event `self.ReceiveTick`
  (params (DeltaSeconds :type "Float (single-precision)"))
  (bind _currentphase (`self.CurrentPhase`))
  ;[1 1 1] Event Tick
  (set `self.LockPlayerInput` false)
  (if (not (`self.MoondialCompleted`))
    (bind _needsupdate (`self.UpdateCurrentPhase` DeltaSeconds))
    (if _needsupdate
      (bind _moonphase (`self.GetPhaseByInteger` (`KismetMathLibrary.FFloor` _currentphase)))
      (bind _moonphase_2 (`self.GetPhaseByInteger` (`KismetMathLibrary.FCeil` _currentphase)))
      (`self.SetPhase` _moonphase _moonphase_2 (mod _currentphase 1.0))
      (set `self.LockPlayerInput` true)
      (`SceneComponent.K2_SetRelativeRotation` (`self.RingPivot`) (`KismetMathLibrary.MakeRotator` 0.0 0.0 (* _currentphase 45.0)) false false)
      (elif (== _currentphase 4.0)
        (set `self.MoondialCompleted` true)
        (`self.PickupLantern`)
        (`self.OnMoonDialCompleted`)))))

(event `/Game/Systems/Mechanics/BP_InteractableInterface.Interact`
  (params (Player :type "/Game/Entities/Player/BP_Player Object Reference"))
  (bind _unlockphase (`self.UnlockPhase`))
  ;[1 1 1] Interact
  (if (or (not (`self.CanInteract`)) (`self.MoondialCompleted`))
    _
    (elif (`self.LanternPlaced`)
      (bind (_moonphase _mooncoin) (`self.GetPhaseByInteger` _unlockphase))
      (bind _success (`self.AttemptCompletePhase` Player _moonphase _mooncoin))
      (if _success
        (`self.DelayInteraction` 1.0)
        (`KismetSystemLibrary.Delay` 0.35)
        (bind _output_get (set `self.UnlockPhase` (+ _unlockphase 1)))
        (`self.NextPhase`)
        (`self.OnMoonCoinPlaced` _output_get))
      (else
        (`self.PlaceLantern` Player)
        (`self.DelayInteraction` 1.0)))))

(event `DelayInteraction`
  (params (Delay :type "Float (double-precision)"))
  ;[1 1 1] Interact
  (set `self.CanInteract` false)
  (`KismetSystemLibrary.Delay` Delay)
  (set `self.CanInteract` true))

(event `PlayerInput`
  (params (LeftRight :type "Float (double-precision)"))
  ;[0.4479 0.1858 0.1411] Player Next Prev
  (if (`self.LockPlayerInput`)
    _
    (elif (> LeftRight 0.0)
      (`self.NextPhase`)
      (elif (< LeftRight 0.0)
        (`self.PrevPhase`)))))

(event `NextPhase`
  (bind _audio (`self.Audio`))
  (bind _returnvalue (+ (`self.prevAudioLevel`) 1.0))
  ;[0.4479 0.1858 0.1411] Player Next Prev
  (`AudioComponent.FadeIn` _audio 0.5 1.0 0.0 "Linear")
  (set `self.GoalPhase` (`KismetMathLibrary.FClamp` (+ (`self.GoalPhase`) 1.0) 0.0 (`KismetMathLibrary.Conv_IntToDouble` (- (`self.UnlockPhase`) 1))))
  (`KismetSystemLibrary.Delay` 4.0)
  (`AudioComponent.FadeOut` _audio 0.5 0.0 "Linear")
  (`AudioParameterControllerInterface.SetFloatParameter` (`/Game/Entities/Gameplay/Items/BP_ItemLantern.LanternNoise` (`self.Lantern`)) "IncreaseMoon" _returnvalue)
  (set `self.prevAudioLevel` _returnvalue))

(event `PrevPhase`
  ;[0.4479 0.1858 0.1411] Player Next Prev
  (`GameplayStatics.PlaySound2D` "/Game/Audio/Gameplay/Scratch/sfx_feedback_stoneGrinding_01.sfx_feedback_stoneGrinding_01" 1.0 1.0 0.0 null null)
  (set `self.GoalPhase` (`KismetMathLibrary.FClamp` (- (`self.GoalPhase`) 1.0) 0.0 (`KismetMathLibrary.Conv_IntToDouble` (- (`self.UnlockPhase`) 1)))))

(event `PlaceLantern`
  (params (Player :type "/Game/Entities/Player/BP_Player Object Reference"))
  (bind _equippeditem_itemname (break `/Game/Entities/Gameplay/Items/S_ItemData` (`/Game/Entities/Player/BP_Player.EquippedItem` Player)))
  (bind _gibbousmoon_coinname (break `/Game/Systems/Level/MoonPhaseData` (`self.GibbousMoon`)))
  (bind _returnvalue (== _equippeditem_itemname _gibbousmoon_coinname))
  ;[1 1 1] Place Lantern
  (`/Engine/EditorBlueprintResources/StandardMacros.DoOnce` false
    (:`Completed`
      (if _returnvalue
        (`/Game/Entities/Player/BP_Player.OnItemInteract` Player "NewEnumerator14")
        (else
          (`/Game/Entities/Player/BP_Player.OnItemInteract` Player "NewEnumerator2")))
      (`KismetSystemLibrary.Delay` 0.6)
      (set `self.LanternPlaced` true)
      (`SceneComponent.SetVisibility` (`self.LanternLight`) true false)
      (for _array_element (`self.GetAttachedActors` Player true false)
        (bind _asbp_item_lantern (cast `/Game/Entities/Gameplay/Items/BP_ItemLantern` _array_element))
        (bind _output_get (set `self.Lantern` _asbp_item_lantern))
        (`self.SetActorScale3D` _output_get (10.0 10.0 10.0))
        (`self.K2_SetActorRelativeRotation` :`self` _output_get)
        (`/Game/Entities/Gameplay/Items/BP_ItemLantern.AttachToActor` _output_get (`self.LanternPivot`) false)
        (`self.SetActorEnableCollision` _output_get false)
        (`KismetSystemLibrary.Delay` 0.2)
        (set `/Game/Entities/Player/BP_Player.hasLantern` false Player)
        (if _returnvalue
          (`/Game/Entities/Player/BP_Player.OnItemEquipped` Player _equippeditem_itemname)
          (else
            (`/Game/Entities/Player/BP_Player.OnItemUnequipped` Player)))))))

(event `PickupLantern`
  (bind _lantern (`self.Lantern`))
  (bind _player (`self.Player`))
  (`SceneComponent.SetVisibility` (`self.LanternLight`) false false)
  (set `/Game/Entities/Gameplay/Items/BP_ItemLantern.CanPickup` true _lantern)
  (`/Game/Systems/Mechanics/BP_InteractableInterface.Interact` _lantern _player)
  (set `/Game/Entities/Player/BP_Player.MOONLANTERNPICKUP` true _player)
  (`/Game/Entities/Player/BP_Player.OnItemFirstPickup` _player "NewEnumerator2")
  (`/Game/Entities/Player/BP_Player.DisableMoondial` _player)
  (`self.DisableInput` _player null)
  (`KismetSystemLibrary.Delay` 2.0)
  (`self.EnableInput` _player null))

(fn `AttemptCompletePhase`
  (params (Player :type "/Game/Entities/Player/BP_Player Object Reference") (Phase :type "/Game/Systems/Level/MoonPhaseData Structure") (PhaseCoin :type "StaticMeshComponent Object Reference"))
  (returns (Success :type Boolean))
  (bind _equippeditem_itemname (break `/Game/Entities/Gameplay/Items/S_ItemData` (`/Game/Entities/Player/BP_Player.EquippedItem` Player)))
  (if (== _equippeditem_itemname Phase_CoinName_2_288596CA42B89737A3C7FCB5656BDE3D)
    (`/Game/Entities/Player/BP_Player.OnItemInteract` Player "NewEnumerator13")
    (`/Game/Entities/Player/BP_Player.RemoveEquippedItem` Player)
    (`SceneComponent.SetVisibility` PhaseCoin true false)
    (return true)
    (else
      (return false))))

(fn `GetPhaseByInteger`
  (params (Int :type Integer))
  (returns (MoonPhase :type "/Game/Systems/Level/MoonPhaseData Structure") (MoonCoin :type "StaticMeshComponent Object Reference"))
  (switch `int` Int
    (:`0`
      (return (`self.FullMoon`) (`self.FullMoonCoin`)))
    (:`1`
      (return (`self.GibbousMoon`) (`self.GibbousMoonCoin`)))
    (:`2`
      (return (`self.HalfMoon`) (`self.HalfMoonCoin`)))
    (:`3`
      (return (`self.CrescentMoon`) (`self.CrescentMoonCoin`)))
    (:`4`
      (return (`self.NewMoon`) (`self.NewMoonCoin`)))))

(fn `GetPrompt`
  (params (player :type "/Game/Entities/Player/BP_Player Object Reference"))
  (returns (inputAction :type "InputAction Object Reference") (actionText :type Text))
  (if (not (`self.MoondialCompleted`))
    (if (`/Game/Entities/Player/BP_Player.hasLantern` player)
      (return "/Game/Entities/Player/Input/IA_Interact.IA_Interact" "place lantern")
      (else
        (bind (_itemequipped _equippeditem) (`/Game/Entities/Player/BP_Player.GetEquippedItem` player))
        (if _itemequipped
          (return "/Game/Entities/Player/Input/IA_Interact.IA_Interact" (`KismetTextLibrary.Conv_StringToText` (`KismetStringLibrary.Concat_StrStr` "place " (break `/Game/Entities/Gameplay/Items/S_ItemData` _equippeditem))))
          (else
            (return null "equip an item to place")))))))

(fn `HideAllPhaseCoins`
  (for _array_element (`|MakeArray` (`self.GibbousMoonCoin`) (`self.HalfMoonCoin`) (`self.CrescentMoonCoin`) (`self.NewMoonCoin`))
    (`SceneComponent.SetVisibility` _array_element false false)))

(fn `SetLightIntensityColor`
  (params (Light :type "LightComponent Object Reference") (Intensity :type "Float (single-precision)") (Color :type "LinearColor Structure"))
  (`LightComponent.SetIntensity` Light Intensity)
  (`LightComponent.SetLightColor` Light Color true))

(fn `SetPhase`
  (params (StartPhase :type "/Game/Systems/Level/MoonPhaseData Structure") (EndPhase :type "/Game/Systems/Level/MoonPhaseData Structure") (Delta :type "Float (double-precision)"))
  (`|ExecutionSequence`
    (:`then_0`
      (`self.K2_SetActorRelativeRotation` (`self.Moon`) (`KismetMathLibrary.RLerp` StartPhase_MoonRotation_33_8D69170649BD9833F03DC4BDF724F9FB EndPhase_MoonRotation_33_8D69170649BD9833F03DC4BDF724F9FB Delta) false false)
      (`self.SetLightIntensityColor` (`Light.LightComponent` (`self.DirLight`)) (`KismetMathLibrary.Lerp` StartPhase_MoonLightIntensity_15_39F2E94E4CC923F387DFFAA4A5D1A9F2 EndPhase_MoonLightIntensity_15_39F2E94E4CC923F387DFFAA4A5D1A9F2 Delta) (`KismetMathLibrary.LinearColorLerp` StartPhase_MoonLightColor_28_320BBDB0429F3F8BCEA246B5F4589848 EndPhase_MoonLightColor_28_320BBDB0429F3F8BCEA246B5F4589848 Delta))
      (`self.SetLightIntensityColor` (`self.LanternLight`) (`KismetMathLibrary.Lerp` StartPhase_LanternLightIntensity_31_28F6FD54438AECF82A4600891C2B2EB6 EndPhase_LanternLightIntensity_31_28F6FD54438AECF82A4600891C2B2EB6 Delta) (`KismetMathLibrary.LinearColorLerp` StartPhase_LanternLightColor_32_0401300743BF3D60882261AB6D9C956A EndPhase_LanternLightColor_32_0401300743BF3D60882261AB6D9C956A Delta)))
    (:`then_1`
      (if (> (mod Delta 1.0) 0.5)
        (for _array_element EndPhase_VineDoorsToOpen_6_B625F1944CA1A4FA1FBDE2854A779074
          (`/Game/Entities/Gameplay/Moondial/BP_VineDoor.OpenVineDoor` _array_element))))))

(fn `UpdateCurrentPhase`
  (params (TimeDelta :type "Float (double-precision)"))
  (returns (NeedsUpdate :type Boolean))
  (if (== (`self.CurrentPhase`) (`self.GoalPhase`))
    (return false)
    (else
      (if (< (`KismetMathLibrary.Abs` (- (`self.CurrentPhase`) (`self.GoalPhase`))) 0.01)
        (set `self.CurrentPhase` (`self.GoalPhase`))
        (elif (< (`self.CurrentPhase`) (`self.GoalPhase`))
          (set `self.CurrentPhase` (+ (`self.CurrentPhase`) (* TimeDelta (`self.UpdateSpeed`))))
          (elif (> (`self.CurrentPhase`) (`self.GoalPhase`))
            (set `self.CurrentPhase` (`self.GoalPhase`))
            (return false)
            (else
              (`KismetSystemLibrary.PrintString` "Unknown Error with Moondial Current Phase???")
              (return false)))))
      (return true))))

(fn `UserConstructionScript`)