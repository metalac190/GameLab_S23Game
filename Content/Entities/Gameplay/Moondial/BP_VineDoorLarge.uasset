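; BP_VineDoorLarge is the large vine door among the Moondial gameplay entities, with animations for closed, opening and open states.
; Three functions each play one non-looping animation directly on the skeletal mesh.
; It holds no trigger or state logic: the event graph is disabled, the construction script only calls its parent, and nothing here calls the animation functions.
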(fn `PlayClosedAnim`
  (`SkeletalMeshComponent.PlayAnimation` (`self.SkeletalMesh`) "/Game/Art/03_Greenhouse/Vine_Doors/HeartCorridor_Door/Anims/Closed.Closed" false))

(fn `PlayOpenAnim`
  (`SkeletalMeshComponent.PlayAnimation` (`self.SkeletalMesh`) "/Game/Art/03_Greenhouse/Vine_Doors/HeartCorridor_Door/Anims/Openned.Openned" false))

(fn `PlayOpeningAnim`
  (`SkeletalMeshComponent.PlayAnimation` (`self.SkeletalMesh`) "/Game/Art/03_Greenhouse/Vine_Doors/HeartCorridor_Door/Anims/Openning.Openning" false))

(fn `UserConstructionScript`
  (`parent.UserConstructionScript`))