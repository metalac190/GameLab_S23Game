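; BP_MoonPhase4 is a Moondial gameplay Blueprint that switches off its accompanying firefly and light effects when interacted with.
; Its InteractResponse sets the FireFlies Niagara spawn rate to zero and hides the Light component, each after a validity check on the referenced object.
; It then calls the parent InteractResponse, and its construction script only calls the parent's.
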(fn `InteractResponse`
  (bind _fireflies (`self.FireFlies`))
  (bind _light (`self.Light`))
  (`/Engine/EditorBlueprintResources/StandardMacros.IsValid` _fireflies
    (:`Is Valid`
      (`FXSystemComponent.SetFloatParameter` (`NiagaraActor.NiagaraComponent` _fireflies) "User.SpawnRate" 0.0))
    (:`Is Not Valid`
      _))
  (`/Engine/EditorBlueprintResources/StandardMacros.IsValid` _light
    (:`Is Valid`
      (`SceneComponent.SetVisibility` (`Light.LightComponent` _light) false true))
    (:`Is Not Valid`
      _))
  (`parent.InteractResponse`))

(fn `UserConstructionScript`
  (`parent.UserConstructionScript`))