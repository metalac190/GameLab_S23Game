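; BP_VineDoor is a vine-covered door in the Moondial gameplay set that opens through its OpenVineDoor event, with no closing logic.
; The event plays the skeletal mesh animation and a timeline that slides the left and right vines apart while disabling both box colliders.
; A DoOnce plays a shrivel sound at the vine offset vector, used as a world location.
; The skeletal mesh hides when the timeline finishes.
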(event `OpenVineDoor`
  (`SkeletalMeshComponent.Play` (`self.SkeletalMesh`) false)
  (bind (_direction _offset) (`Timeline|VineDoorTimeline`)
    (:`Update`
      (bind _returnvalue (* _offset 60.0))
      (bind _returnvalue_2 (`KismetMathLibrary.MakeVector` 0.0 _returnvalue))
      (`SceneComponent.K2_SetRelativeLocation` (`self.LeftVine`) _returnvalue_2 false false)
      (`SceneComponent.K2_SetRelativeLocation` (`self.RightVine`) (`KismetMathLibrary.MakeVector` 0.0 (- 0.0 _returnvalue)) false false)
      (`PrimitiveComponent.SetCollisionEnabled` (`self.Box`) "NoCollision")
      (`PrimitiveComponent.SetCollisionEnabled` (`self.Box1`) "NoCollision")
      (`/Engine/EditorBlueprintResources/StandardMacros.DoOnce` false
        (:`Completed`
          (`GameplayStatics.PlaySoundAtLocation` "/Game/Audio/Gameplay/Cues/sfx_feedback_vineShrivel_01.sfx_feedback_vineShrivel_01" _returnvalue_2 (struct) 1.0 1.0 0.0 null null null null))))
    (:`Finished`
      (`SceneComponent.SetVisibility` (`self.SkeletalMesh`) false true))))

(fn `UserConstructionScript`)