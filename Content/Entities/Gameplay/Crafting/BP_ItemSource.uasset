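; BP_ItemSource is an interactable crafting item source that gives its item to the player's inventory.
; It copies ItemData from its Item on BeginPlay, then on Interact passes it to BPCInventory's AddToInventory on BP_Player.
; The result sets ItemInUse, and while that is true further interactions only print a debug message.
; The EquippedIndex check has empty branches, and a GetStoredItem lookup is left unconnected.
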(event `self.ReceiveBeginPlay`
  (set `self.ItemData` (`/Game/Entities/Gameplay/Items/BP_ITEM_MASTER.ItemData` (`self.Item`))))

(event `/Game/Systems/Mechanics/BP_InteractableInterface.Interact`
  (params (Player :type "/Game/Entities/Player/Blueprints/BP_Player Object Reference"))
  (bind _asbp_player (cast `/Game/Entities/Player/Blueprints/BP_Player` (`GameplayStatics.GetPlayerPawn` 0)))
  (if (>= (`/Game/Entities/Player/Blueprints/BP_Player.EquippedIndex` _asbp_player) 0)
    _
    (else
      _))
  (if (`self.ItemInUse`)
    (`KismetSystemLibrary.PrintString` "Alreadying Gradbbed this item")
    (else
      (bind _itemadded (`/Game/Entities/Player/Blueprints/BPC_Inventory.AddToInventory` (`/Game/Entities/Player/Blueprints/BP_Player.BPC_Inventory` _asbp_player) (`self.ItemData`)))
      (set `self.ItemInUse` _itemadded))))

(fn `UserConstructionScript`)