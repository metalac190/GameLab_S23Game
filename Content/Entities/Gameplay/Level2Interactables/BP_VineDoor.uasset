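; BP_VineDoor is a Level 2 interactable vine door that presents itself as something the player can burn.
; GetPrompt checks the player's equipped item by name and offers the interact input only for flint & steel.
; Any other item gets a "can't ignite" message, and empty hands get a flammability hint.
; The Interact event is an empty stub, so no burning or opening logic exists here.
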(event `/Game/Systems/Mechanics/BP_InteractableInterface.Interact`
  (params (Player :type "/Game/Entities/Player/BP_Player Object Reference")))

(fn `GetPrompt`
  (params (player :type "/Game/Entities/Player/BP_Player Object Reference"))
  (returns (inputAction :type "InputAction Object Reference") (actionText :type Text))
  (bind (_itemequipped _equippeditem) (`/Game/Entities/Player/BP_Player.GetEquippedItem` player))
  (if _itemequipped
    (if (== (break `/Game/Entities/Gameplay/Items/S_ItemData` _equippeditem) "flint & steel")
      (return "/Game/Entities/Player/Input/IA_Interact.IA_Interact" "ingite with flint & steel")
      (else
        (return null (`KismetTextLibrary.Conv_StringToText` (`KismetStringLibrary.Concat_StrStr` (break `/Game/Entities/Gameplay/Items/S_ItemData` _equippeditem) " can't ingite this")))))
    (else
      (return null "this looks like it will burn easily"))))

(fn `UserConstructionScript`
  (`parent.UserConstructionScript`))