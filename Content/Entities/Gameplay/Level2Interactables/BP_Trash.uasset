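; BP_Trash is a Level 2 interactable that lets the player throw away their equipped item if its name is in AllowedObjects.
; Interacting passes the item to the Crafter's BPCCrafter to reset its item source, fires the player's any-interact call and removes the item.
; GetPrompt shows whether disposal is possible, offering the interact input only for allowed items.
; An unset Crafter falls back to the BP_MortarAndPestle found at BeginPlay.
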(event `self.ReceiveBeginPlay`
  ;[1 1 1] Small hack so I didn't have to touch the level
  (`/Engine/EditorBlueprintResources/StandardMacros.IsValid` (`self.crafter`)
    (:`Is Not Valid`
      (bind _returnvalue (`GameplayStatics.GetActorOfClass` "/Game/Entities/Gameplay/Level2Interactables/BP_MortarAndPestle.BP_MortarAndPestle_C"))
      (set `self.crafter` _returnvalue))))

(event `/Game/Systems/Mechanics/BP_InteractableInterface.Interact`
  (params (Player :type "/Game/Entities/Player/BP_Player Object Reference"))
  (bind (_itemequipped _equippeditem) (`/Game/Entities/Player/BP_Player.GetEquippedItem` Player))
  (if _itemequipped
    (if (`BlueprintSetLibrary.Set_Contains` (`self.AllowedObjects`) (`.ItemName_18_CD23B635439CECA1569C62A2D3CDE386` (break `/Game/Entities/Gameplay/Items/S_ItemData` _equippeditem)))
      (`/Game/Systems/Mechanics/Crafting/BPC_Crafter.ResetItemSources` (`/Game/Entities/Gameplay/Level2Interactables/BP_MortarAndPestle.BPC_Crafter` (`self.crafter`)) (`|MakeArray` _equippeditem))
      (`/Game/Entities/Player/BP_Player.OnAnyInteract` Player)
      (`/Game/Entities/Player/BP_Player.RemoveEquippedItem` Player))))

(fn `GetPrompt`
  (params (player :type "/Game/Entities/Player/BP_Player Object Reference"))
  (returns (inputAction :type "InputAction Object Reference") (actionText :type Text))
  (bind (_itemequipped _equippeditem) (`/Game/Entities/Player/BP_Player.GetEquippedItem` player))
  (if _itemequipped
    (if (`BlueprintSetLibrary.Set_Contains` (`self.AllowedObjects`) (break `/Game/Entities/Gameplay/Items/S_ItemData` _equippeditem))
      (return "/Game/Entities/Player/Input/IA_Interact.IA_Interact" (`KismetTextLibrary.Conv_StringToText` (`KismetStringLibrary.Concat_StrStr` "throw away " (break `/Game/Entities/Gameplay/Items/S_ItemData` _equippeditem)))) ; tell the player they can do this action
      (else
        (return null "you can't throw this item away") ; Inform the player this object is not meant to be destroyed
      ))
    (else
      (return null "Equip an item to throw away") ; Just display action text by not selecting an input action,\nas pressing interact will not do anything
    )))

(fn `UserConstructionScript`)