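; Level 2 mortar and pestle crafting station where the player adds equipped items, crafts and collects the result.
; Interact takes a waiting output into the inventory, crafts when inputs are full, or feeds the equipped item to BPCCrafter.
; SetMeshes mirrors crafter data as item actors at spot transforms and can signal charm-crafted success.
; Tick polls for missing item actors to clear their crafter data, while GetPrompt supplies state-dependent interaction text.
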(event `self.ReceiveTick`
  (params (DeltaSeconds :type "Float (single-precision)"))
  (`self.CheckPickUp`))

(event `self.ReceiveBeginPlay`
  (set `self.Input Spots` (`|MakeArray` (`SceneComponent.K2_GetComponentToWorld` (`self.Input Spot 1`)) (`SceneComponent.K2_GetComponentToWorld` (`self.Input Spot 2`))))
  (`KismetArrayLibrary.Array_Resize` (`self.Inputs`) (`/Game/Systems/Mechanics/Crafting/BPC_Crafter.Max Items` (`self.BPC_Crafter`)))
  (bind _asbp_player (cast `/Game/Entities/Player/BP_Player` (`GameplayStatics.GetPlayerPawn` 0)))
  (set `self.BP_Player` _asbp_player))

(event `/Game/Systems/Mechanics/BP_InteractableInterface.Interact`
  (params (Player :type "/Game/Entities/Player/BP_Player Object Reference"))
  (bind _output_item_itemname (break `/Game/Entities/Gameplay/Items/S_ItemData` (`/Game/Systems/Mechanics/Crafting/BPC_Crafter.Output Item` (`self.BPC_Crafter`))))
  (if (not (`KismetStringLibrary.IsEmpty` _output_item_itemname))
    (bind _itemadded (`/Game/Systems/Player/BPC_Inventory.AddToInventory` (`/Game/Entities/Player/BP_Player.BPC_Inventory` (`self.BP_Player`)) (`/Game/Systems/Mechanics/Crafting/BPC_Crafter.Output Item` (`self.BPC_Crafter`))))
    (if _itemadded
      (set `/Game/Systems/Mechanics/Crafting/BPC_Crafter.Output Item` (struct) (`self.BPC_Crafter`)))
    (`self.SetMeshes`)
    (else
      (bind _status (`self.AreInputsFull`))
      (if _status
        (`/Game/Systems/Mechanics/Crafting/BPC_Crafter.Craft` (`self.BPC_Crafter`) false)
        (`self.SetMeshes`)
        (else
          ;[1 1 1] Craft
          (bind (_itemequipped _equippeditem) (`/Game/Entities/Player/BP_Player.GetEquippedItem` (`self.BP_Player`)))
          (if _itemequipped
            (`GameplayStatics.PlaySoundAtLocation` "/Game/Audio/Gameplay/Cues/sfx_feedback_mortarPestle_01.sfx_feedback_mortarPestle_01" (`self.K2_GetActorLocation`) (struct) 1.0 1.0 0.0 null null null null)
            (bind _itemadded_2 (`/Game/Systems/Mechanics/Crafting/BPC_Crafter.Add Item` (`self.BPC_Crafter`) _equippeditem))
            (if _itemadded_2
              (`/Game/Entities/Player/BP_Player.RemoveEquippedItem` (`self.BP_Player`))
              (`self.SetMeshes`))
            (else
              (`KismetSystemLibrary.PrintString` "Select an item to craft with!"))))))))

(fn `AreInputsFull`
  (returns (status :type Boolean))
  (for _array_element (`self.Inputs`)
    (if (not (`KismetSystemLibrary.IsValid` _array_element))
      (return false)))
  (return true))

(fn `CheckPickUp`
  (bind _input_items (`/Game/Systems/Mechanics/Crafting/BPC_Crafter.Input Items` (`self.BPC_Crafter`)))
  (bind _output_item_itemname (break `/Game/Entities/Gameplay/Items/S_ItemData` (`/Game/Systems/Mechanics/Crafting/BPC_Crafter.Output Item` (`self.BPC_Crafter`))))
  (`|ExecutionSequence`
    (:`then_0`
      ;[1 1 1] Check Inputs
      (for (_array_element _array_index) (`self.Inputs`)
        (bind _output_itemname (break `/Game/Entities/Gameplay/Items/S_ItemData` (`|GetArrayItem` _input_items _array_index)))
        (if (and (not (`KismetSystemLibrary.IsValid` _array_element)) (< _array_index (`KismetArrayLibrary.Array_Length` _input_items)) (not (`KismetStringLibrary.IsEmpty` _output_itemname)))
          (`KismetArrayLibrary.Array_Remove` (`/Game/Systems/Mechanics/Crafting/BPC_Crafter.Input Items` (`self.BPC_Crafter`)) _array_index)
          (`self.SetMeshes` :!label _label))))
    (:`then_1`
      ;[1 1 1] Check Output
      (if (and (not (`KismetSystemLibrary.IsValid` (`self.Output`))) (not (`KismetStringLibrary.IsEmpty` _output_item_itemname)))
        (set `/Game/Systems/Mechanics/Crafting/BPC_Crafter.Output Item` (struct) (`self.BPC_Crafter`))
        (goto _label)))))

(fn `CreateItem`
  (params (SpawnPoint :type "Transform Structure") (Data :type "/Game/Entities/Gameplay/Items/S_ItemData Structure"))
  (returns (NewParam :type "/Game/Entities/Gameplay/Items/BP_ITEM_MASTER Object Reference"))
  (bind _returnvalue (`|SpawnActorFromClass` "/Game/Entities/Gameplay/Items/BP_ITEM_MASTER.BP_ITEM_MASTER_C" SpawnPoint "Undefined" "OverrideRootScale" null null))
  (`/Game/Entities/Gameplay/Items/BP_ITEM_MASTER.Set Data` _returnvalue Data)
  (return _returnvalue))

(fn `GetPrompt`
  (params (player :type "/Game/Entities/Player/BP_Player Object Reference"))
  (returns (inputAction :type "InputAction Object Reference") (actionText :type Text))
  (bind _output_item_itemname (break `/Game/Entities/Gameplay/Items/S_ItemData` (`/Game/Systems/Mechanics/Crafting/BPC_Crafter.Output Item` (`self.BPC_Crafter`))))
  (if (`KismetSystemLibrary.IsValid` (`self.Output`))
    (return "/Game/Entities/Player/Input/IA_Interact.IA_Interact" (`KismetTextLibrary.Conv_StringToText` (`KismetStringLibrary.Concat_StrStr` "pickup " _output_item_itemname)))
    (else
      (bind _status (`self.AreInputsFull`))
      (if _status
        (return "/Game/Entities/Player/Input/IA_Interact.IA_Interact" "craft")
        (else
          (bind (_itemequipped _equippeditem) (`/Game/Entities/Player/BP_Player.GetEquippedItem` (`self.BP_Player`)))
          (if _itemequipped
            (if (`KismetArrayLibrary.Array_Contains` (`/Game/Systems/Mechanics/Crafting/BPC_Crafter.allowedInputs` (`self.BPC_Crafter`)) (break `/Game/Entities/Gameplay/Items/S_ItemData` _equippeditem))
              (return "/Game/Entities/Player/Input/IA_Interact.IA_Interact" (`KismetTextLibrary.Conv_StringToText` (`KismetStringLibrary.Concat_StrStr` "add " (break `/Game/Entities/Gameplay/Items/S_ItemData` _equippeditem) " to mortar & pestle")))
              (else
                (return null "You can't put this in the mortar &  pestle")))
            (else
              (return null "Equip an item to add to mortar & pestle"))))))))

(fn `SetMeshes`
  (locals (mesh :type "StaticMeshComponent Object Reference"))
  (bind _output_item (`/Game/Systems/Mechanics/Crafting/BPC_Crafter.Output Item` (`self.BPC_Crafter`)))
  ;[1 1 1] Manage Inputs
  (for (_array_element _array_index) (`self.Inputs`)
    (if (< _array_index (`KismetArrayLibrary.Array_Length` (`/Game/Systems/Mechanics/Crafting/BPC_Crafter.Input Items` (`self.BPC_Crafter`))))
      (bind _returnvalue (`KismetSystemLibrary.IsValid` _array_element))
      (if _returnvalue
        (bind _output (`|GetArrayItem` (`/Game/Systems/Mechanics/Crafting/BPC_Crafter.Input Items` (`self.BPC_Crafter`)) _array_index))
        (bind _destroyeditem (`/Game/Entities/Gameplay/Items/BP_ITEM_MASTER.Set Data` _array_element _output))
        (if _destroyeditem
          (`KismetArrayLibrary.Array_Set` (`self.Inputs`) _array_index :!label _label))
        (else
          (bind _itemactor (`/Game/Systems/Utility/ItemMacroLibrary.CreateItemInstance` _output (`|GetArrayItem` (`self.Input Spots`) _array_index))
            (:`OutExec`
              (`KismetArrayLibrary.Array_Set` (`self.Inputs`) _array_index _itemactor)))))
      (elif _returnvalue
        (`self.K2_DestroyActor` _array_element)
        (goto _label))))
  ;[1 1 1] Manage Outputs
  (if (`KismetSystemLibrary.IsValid` (`self.Output`))
    (bind _destroyeditem_2 (`/Game/Entities/Gameplay/Items/BP_ITEM_MASTER.Set Data` (`self.Output`) _output_item))
    (if _destroyeditem_2
      (set `self.Output` null)
      (`self.CharmCraftedSuccess`)
      (`KismetSystemLibrary.PrintString` "Charm Crafted Success"))
    (else
      (bind _itemactor_2 (`/Game/Systems/Utility/ItemMacroLibrary.CreateItemInstance` _output_item (`SceneComponent.K2_GetComponentToWorld` (`self.Output Spot`)))
        (:`OutExec`
          (set `self.Output` _itemactor_2))))))

(fn `UserConstructionScript`)