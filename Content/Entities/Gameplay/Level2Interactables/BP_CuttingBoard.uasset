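; BP_CuttingBoard is a Level 2 interactable board where the player places equipped items.
; It caches up to four spot transforms on BeginPlay, trimmed to MaxItems, with a parallel Items array tracking occupancy.
; Interact spawns the equipped item at the first free spot and removes it from the player, or prints that it is full.
; GetPrompt shows a place or equip-first message.
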(event `self.ReceiveBeginPlay`
  (bind _output_get (set `self.Input Spots` (`|MakeArray` (`SceneComponent.K2_GetComponentToWorld` (`self.Spot 1`)) (`SceneComponent.K2_GetComponentToWorld` (`self.Spot 2`)) (`SceneComponent.K2_GetComponentToWorld` (`self.Spot 3`)) (`SceneComponent.K2_GetComponentToWorld` (`self.Spot 4`)))))
  (`KismetArrayLibrary.Array_Resize` _output_get (`self.maxItems`))
  (`KismetArrayLibrary.Array_Resize` (`self.Items`) (`KismetArrayLibrary.Array_Length` (`self.Input Spots`)))
  (bind _asbp_player (cast `/Game/Entities/Player/BP_Player` (`GameplayStatics.GetPlayerPawn` 0)))
  (set `self.BP_Player` _asbp_player))

(event `/Game/Systems/Mechanics/BP_InteractableInterface.Interact`
  (params (Player :type "/Game/Entities/Player/BP_Player Object Reference"))
  (bind (_itemequipped _equippeditem) (`/Game/Entities/Player/BP_Player.GetEquippedItem` Player))
  (if _itemequipped
    (bind _index (`self.GetFirstIndex`))
    (if (>= _index 0)
      (bind _itemactor (`/Game/Systems/Utility/ItemMacroLibrary.CreateItemInstance` _equippeditem (`|GetArrayItem` (`self.Input Spots`) _index))
        (:`OutExec`
          (`KismetArrayLibrary.Array_Set` (`self.Items`) _index _itemactor)
          (`/Game/Entities/Player/BP_Player.RemoveEquippedItem` (`self.BP_Player`))
          (`/Game/Entities/Player/BP_Player.RemoveEquippedItem` Player)))
      (else
        (`KismetSystemLibrary.PrintString` "Table is full")))))

(fn `GetFirstIndex`
  (returns (Index :type Integer))
  (for (_array_element _array_index) (`self.Items`)
    (if (not (`KismetSystemLibrary.IsValid` _array_element))
      (return _array_index)))
  (return -1))

(fn `GetPrompt`
  (params (player :type "/Game/Entities/Player/BP_Player Object Reference"))
  (returns (inputAction :type "InputAction Object Reference") (actionText :type Text))
  (bind (_itemequipped _equippeditem) (`/Game/Entities/Player/BP_Player.GetEquippedItem` player))
  (if (not _itemequipped)
    (return null "Equip an item to place here")
    (else
      (return "/Game/Entities/Player/Input/IA_Interact.IA_Interact" (`KismetTextLibrary.Conv_StringToText` (`KismetStringLibrary.Concat_StrStr` "place " (break `/Game/Entities/Gameplay/Items/S_ItemData` _equippeditem)))))))

(fn `UserConstructionScript`)