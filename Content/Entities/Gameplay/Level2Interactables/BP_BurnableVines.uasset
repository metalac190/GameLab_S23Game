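; Interactable burnable vines that block the player until ignited with an equipped flint & steel, with prompts reflecting the held item.
; Ignition plays audio and a timeline that slides SourcePoint toward StopPosition, feeding its position to the PC_BurnAway parameter collection and burn-away Niagara effect.
; Past the ClearDoorAfter threshold the collider is removed and audio stops, then the actor destroys itself when the timeline finishes.
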(event `self.ReceiveBeginPlay`
  (`self.SetFireSourcePoint`)
  (if (`self.NoSmoke`)
    (`ActorComponent.K2_DestroyComponent` (`self.NS_BurnAway`))))

(event `/Game/Systems/Mechanics/BP_InteractableInterface.Interact`
  (params (Player :type "/Game/Entities/Player/BP_Player Object Reference"))
  (bind (_itemequipped _equippeditem) (`/Game/Entities/Player/BP_Player.GetEquippedItem` Player))
  (if _itemequipped
    (if (== (break `/Game/Entities/Gameplay/Items/S_ItemData` _equippeditem) "flint & steel")
      (`/Engine/EditorBlueprintResources/StandardMacros.DoOnce` false
        (:`Completed`
          (`/Game/Entities/Player/BP_Player.OnItemInteract` Player "NewEnumerator10")
          (`self.Ignite`))))))

(event `Ignite`
  (`self.Ignited`)
  (`self.SetFireRadius` (`self.StartRadius`))
  (set `self.bIsBurning` true)
  (`AudioComponent.Play` (`self.Audio`) 0.0)
  (set `self.StartPosition` (`SceneComponent.RelativeLocation` (`self.SourcePoint`)))
  (bind (_direction _alpha) (`Timeline|IgniteTimline` :!via `PlayFromStart`)
    (:`Update`
      (`|ExecutionSequence`
        (:`then_1`
          ;[1 1 1] Move Source Point
          (`SceneComponent.K2_SetRelativeLocation` (`self.SourcePoint`) (`KismetMathLibrary.VLerp` (`self.StartPosition`) (`self.StopPosition`) _alpha) false false)
          (`self.SetFireSourcePoint`))
        (:`then_2`
          (if (> _alpha (`self.ClearDoorAfter%`))
            (`/Engine/EditorBlueprintResources/StandardMacros.DoOnce` false
              (:`Completed`
                (`ActorComponent.K2_DestroyComponent` (`self.Collider`))
                (`AudioComponent.Stop` (`self.Audio`))))))))
    (:`Finished`
      (`self.K2_DestroyActor`))))

(fn `GetPrompt`
  (params (player :type "/Game/Entities/Player/BP_Player Object Reference"))
  (returns (inputAction :type "InputAction Object Reference") (actionText :type Text))
  (if (`self.bIsBurning`)
    (return null "")
    (else
      (bind (_itemequipped _equippeditem) (`/Game/Entities/Player/BP_Player.GetEquippedItem` player))
      (if _itemequipped
        (if (== (break `/Game/Entities/Gameplay/Items/S_ItemData` _equippeditem) "flint & steel")
          (return "/Game/Entities/Player/Input/IA_Interact.IA_Interact" "ingite with flint & steel")
          (else
            (return null (`KismetTextLibrary.Conv_StringToText` (`KismetStringLibrary.Concat_StrStr` (break `/Game/Entities/Gameplay/Items/S_ItemData` _equippeditem) " can't ingite this")))))
        (else
          (return null "this looks like it will burn easily"))))))

(fn `SetFireRadius`
  (params (radius :type "Float (double-precision)"))
  (`KismetMaterialLibrary.SetScalarParameterValue` "/Game/VFX/Gameplay/Burn_Away/PC_BurnAway.PC_BurnAway" "Radius" radius)
  (`NiagaraComponent.SetVariableFloat` (`self.NS_BurnAway`) "User.Sphere Radius" radius))

(fn `SetFireSourcePoint`
  (bind _sourcepoint (`self.SourcePoint`))
  (`NiagaraComponent.SetVariableVec3` (`self.NS_BurnAway`) "Origin Offset" (`SceneComponent.RelativeLocation` _sourcepoint))
  (`KismetMaterialLibrary.SetVectorParameterValue` "/Game/VFX/Gameplay/Burn_Away/PC_BurnAway.PC_BurnAway" "location" (`KismetMathLibrary.Conv_VectorToLinearColor` (`SceneComponent.K2_GetComponentLocation` _sourcepoint))))

(fn `UserConstructionScript`
  (`self.SetFireSourcePoint`)
  (`self.SetFireRadius` (`self.StartRadius`))
  (`SceneComponent.SetWorldScale3D` (`self.NS_BurnAway`) (1.0 1.0 1.0)))