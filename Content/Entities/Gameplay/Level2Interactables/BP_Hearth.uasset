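; BP_Hearth is a Level 2 puzzle interactable that takes items in sequence: kindling, flint and steel, then adder stone.
; TryUnlock matches the equipped item to the first Keys entry and removes it, consuming the item while EatKey is set.
; The remaining key count drives each stage's prompts, visuals, fire effects and event dispatchers.
; The adder stone stays blocked until EnableUsingAdderstone is called, and igniting clears EatKey so the stone is kept.
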(event `/Game/Systems/Mechanics/BP_InteractableInterface.Interact`
  (params (Player :type "/Game/Entities/Player/BP_Player Object Reference"))
  (bind _bp_magicalcharmkindling (`self.BP_MagicalCharmKindling`))
  (bind _returnvalue (`SceneComponent.K2_GetComponentLocation` _bp_magicalcharmkindling))
  (if (not (and (> (`KismetArrayLibrary.Array_Length` (`self.Keys`)) 0) (not (`self.canUseAdderStone`)) (== (`|GetArrayItem` (`self.Keys`)) "adder stone")))
    (bind _used_key (`self.TryUnlock` Player))
    (if _used_key
      (switch `int` (`KismetArrayLibrary.Array_Length` (`self.Keys`))
        (:`0`
          (`/Engine/EditorBlueprintResources/StandardMacros.DoOnce` false
            (:`Completed`
              (`self.AdderStoneOnFire`))))
        (:`1`
          (`/Game/Systems/Utility/ItemMacroLibrary.PlayFlint&SteelMontage` Player "/Game/Art/_Global/First_Person_Hands/Anim/Flint_n_Steel_UseFinal_Montage.Flint_n_Steel_UseFinal_Montage"
            (:`On Completed`
              (`SceneComponent.SetVisibility` _bp_magicalcharmkindling true false) ; Enable Kindling Visual
              (`ActorComponent.Activate` (`self.NS_FireFairy`) false) ; Fire on
              (`GameplayStatics.PlaySoundAtLocation` "/Game/Audio/Gameplay/waves/sfx_feedback_lightFire_01.sfx_feedback_lightFire_01" _returnvalue (struct) 1.0 1.0 0.0 null null null null)
              (`AudioComponent.FadeIn` (`self.amb`) 0.2 1.0 0.0 "Linear")
              (`self.MagicalFireLit`)
              (set `self.eatKey` false))))
        (:`2`
          (`KismetSystemLibrary.Delay` 0.2)
          (`SceneComponent.SetVisibility` _bp_magicalcharmkindling true true) ; Add magic charm kindling
          (`GameplayStatics.PlaySoundAtLocation` "/Game/Audio/Gameplay/waves/sfx_feedback_fireFlare_01.sfx_feedback_fireFlare_01" _returnvalue (struct) 1.0 1.0 0.0 null null null null))))))

(event `Enable Using Adderstone`
  (set `self.canUseAdderStone` true))

(fn `GetPrompt`
  (params (player :type "/Game/Entities/Player/BP_Player Object Reference"))
  (returns (inputAction :type "InputAction Object Reference") (actionText :type Text))
  (bind _output (`|GetArrayItem` (`self.Keys`)))
  (bind (_itemequipped _equippeditem) (`/Game/Entities/Player/BP_Player.GetEquippedItem` player))
  (if _itemequipped
    ;[1 1 1] Item Equiped
    (switch `int` (`KismetArrayLibrary.Array_Length` (`self.Keys`))
      (:`0`
        _)
      (:`1`
        (bind _returnvalue (== _output (break `/Game/Entities/Gameplay/Items/S_ItemData` _equippeditem)))
        (if (and _returnvalue (`self.canUseAdderStone`))
          (return "/Game/Entities/Player/Input/IA_Interact.IA_Interact" "use adder stone")
          (else
            _)))
      (:`2`
        (if _returnvalue
          (return "/Game/Entities/Player/Input/IA_Interact.IA_Interact" "ignite")
          (else
            (return null "need something to ingite"))))
      (:`3`
        (if _returnvalue
          (return "/Game/Entities/Player/Input/IA_Interact.IA_Interact" (`KismetTextLibrary.Conv_StringToText` (`KismetStringLibrary.Concat_StrStr` "add " _output " to hearth")))
          (else
            (return null "this isn't a good fire source")))))
    (return null "")
    (else
      ;[1 1 1] No Item Equipped
      (switch `int` (`KismetArrayLibrary.Array_Length` (`self.Keys`))
        (:`0`
          _)
        (:`1`
          _)
        (:`2`
          (return null "need something to ignite this"))
        (:`3`
          (return null "need a firesource")))
      (return null ""))))

(fn `TryUnlock`
  (params (player :type "/Game/Entities/Player/BP_Player Object Reference"))
  (returns (`Used key` :type Boolean))
  (if (`KismetArrayLibrary.Array_IsEmpty` (`self.Keys`))
    (return true)
    (else
      (bind (_itemequipped _equippeditem) (`/Game/Entities/Player/BP_Player.GetEquippedItem` player))
      (if _itemequipped
        (if (== (`.ItemName_18_CD23B635439CECA1569C62A2D3CDE386` (break `/Game/Entities/Gameplay/Items/S_ItemData` _equippeditem)) (`|GetArrayItem` (`self.Keys`)))
          (`self.UsedItem` _equippeditem)
          (`/Game/Entities/Player/BP_Player.OnFinalFlintSteelInteract` player)
          (if (`self.eatKey`)
            (`/Game/Entities/Player/BP_Player.OnItemInteract` player "NewEnumerator11")
            (`/Game/Entities/Player/BP_Player.RemoveEquippedItem` player))
          (`KismetArrayLibrary.Array_Remove` (`self.Keys`))
          (return true)
          (else
            _)))
      (`KismetSystemLibrary.PrintString` "Key doesn't unlock")
      (return false))))

(fn `UserConstructionScript`)