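; Lockable gate door that opens on interaction or, optionally, as soon as it is unlocked, and supplies player prompts for its state.
; Opening sets a flag on the ABP_Gate anim blueprint, stops the idle sound and plays a one-time open sound after a short delay.
; ShakeGate plays a shake montage between pausing and resuming the idle sound.
; An older timeline rotation, the only setter of DoorOpen, is disconnected.
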(event `self.ReceiveBeginPlay`
  (bind _asabp_gate (cast `/Game/VFX/Gameplay/Level1_Gate/Model/ABP_Gate` (`SkeletalMeshComponent.GetAnimInstance` (`self.SkeletalMesh`))))
  (set `self.ABP` _asabp_gate)
  (`AudioComponent.Play` (`self.idleSFX`) 0.0))

(event `/Game/Systems/Mechanics/BP_InteractableInterface.Interact`
  (params (Player :type "/Game/Entities/Player/BP_Player Object Reference"))
  ;[1 1 1] Interact -- Hook up to Player Interactable Interface Eventually
  (if (`self.DoorOpen`)
    _
    (elif (not (`self.Locked`))
      (`self.OpenDoor`))))

(event `OpenDoor`
  (set `/Game/VFX/Gameplay/Level1_Gate/Model/ABP_Gate.opened` true (`self.ABP`))
  (`AudioComponent.Stop` (`self.idleSFX`))
  (`KismetSystemLibrary.Delay` 0.2)
  (`/Engine/EditorBlueprintResources/StandardMacros.DoOnce` false
    (:`Completed`
      (`GameplayStatics.PlaySoundAtLocation` "/Game/Audio/Gameplay/waves/sfx_feedback_doorOpen_01.sfx_feedback_doorOpen_01" (`SceneComponent.K2_GetComponentLocation` (`self.DefaultSceneRoot`)) (struct) 1.0 1.0 0.0 null null null null))))

(event `ShakeGate`
  (`AudioComponent.Stop` (`self.idleSFX`))
  (`|PlayMontage` (`self.SkeletalMesh`) "/Game/VFX/Gameplay/Level1_Gate/Model/Anims/Level_One_Gate_root_Interact_Shake_Montage.Level_One_Gate_root_Interact_Shake_Montage"
    (:`then`
      (`AudioComponent.Play` (`self.idleSFX`) 0.0))))

(fn `GetPrompt`
  (params (player :type "/Game/Entities/Player/BP_Player Object Reference"))
  (returns (inputAction :type "InputAction Object Reference") (actionText :type Text))
  (if (`self.Locked`)
    (return null "The door is locked")
    (elif (`self.DoorOpen`)
      (return "/Game/Entities/Player/Input/IA_Interact.IA_Interact" "close")
      (else
        (return "/Game/Entities/Player/Input/IA_Interact.IA_Interact" "open")))))

(fn `SetLocked`
  (params (Locked :type Boolean))
  (bind _output_get (set `self.Locked` Locked))
  (if (and (not _output_get) (`self.OpenOnUnlocked`))
    (`self.OpenDoor`)))

(fn `UserConstructionScript`)