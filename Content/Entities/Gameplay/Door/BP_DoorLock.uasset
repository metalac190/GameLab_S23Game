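; BP_DoorLock is an interactable lock that keeps its linked door locked until the player uses the required keys.
; Interacting compares the equipped item's name to the first entry in Keys, so keys go in order, firing UsedKey and optionally consuming the item.
; Once Keys is empty, a timeline scales the lock, then unlocks the door and destroys the actor.
; GetPrompt supplies interaction text based on the equipped item.
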(event `self.ReceiveBeginPlay`
  (if (`KismetSystemLibrary.IsValid` (`self.Door`))
    (`/Game/Entities/Gameplay/Door/BP_Door.SetLocked` (`self.Door`) true)))

(event `/Game/Systems/Mechanics/BP_InteractableInterface.Interact`
  (params (Player :type "/Game/Entities/Player/BP_Player Object Reference"))
  (bind _unlocked (`self.TryUnlock` Player))
  (if _unlocked
    (`self.MeltLock`)))

(event `MeltLock`
  ;[1 1 1] Melt Lock
  (bind (_direction _scaletrack) (`Timeline|MeltLockTimeline`)
    (:`Update`
      (`SceneComponent.SetWorldScale3D` (`self.DefaultSceneRoot`) (`KismetMathLibrary.Conv_DoubleToVector` _scaletrack)))
    (:`Finished`
      (if (`KismetSystemLibrary.IsValid` (`self.Door`))
        (`/Game/Entities/Gameplay/Door/BP_Door.SetLocked` (`self.Door`) false))
      (`KismetSystemLibrary.PrintString` "Door Unlocked")
      (`self.K2_DestroyActor`))))

(fn `GetPrompt`
  (params (player :type "/Game/Entities/Player/BP_Player Object Reference"))
  (returns (inputAction :type "InputAction Object Reference") (actionText :type Text))
  (bind (_itemequipped _equippeditem) (`/Game/Entities/Player/BP_Player.GetEquippedItem` player))
  (if _itemequipped
    (return "/Game/Entities/Player/Input/IA_Interact.IA_Interact" (`KismetTextLibrary.Conv_StringToText` (`KismetStringLibrary.Concat_StrStr` "try to unlock with " (break `/Game/Entities/Gameplay/Items/S_ItemData` _equippeditem))))
    (else
      (return null "equip an item to unlock with"))))

(fn `TryUnlock`
  (params (player :type "/Game/Entities/Player/BP_Player Object Reference"))
  (returns (unlocked :type Boolean))
  (bind _keys (`self.Keys`))
  (if (`KismetArrayLibrary.Array_IsEmpty` (`self.Keys`))
    (return true)
    (else
      (bind (_itemequipped _equippeditem) (`/Game/Entities/Player/BP_Player.GetEquippedItem` player))
      (if _itemequipped
        (if (== (`.ItemName_18_CD23B635439CECA1569C62A2D3CDE386` (break `/Game/Entities/Gameplay/Items/S_ItemData` _equippeditem)) (`|GetArrayItem` (`self.Keys`)))
          (`self.UsedKey` _equippeditem)
          (if (`self.eatKey`)
            (`/Game/Entities/Player/BP_Player.RemoveEquippedItem` player))
          (`KismetArrayLibrary.Array_Remove` _keys)
          (return (`KismetArrayLibrary.Array_IsEmpty` _keys))
          (else
            _)))
      (`KismetSystemLibrary.PrintString` "Key doesn't unlock")
      (return false))))

(fn `UserConstructionScript`)