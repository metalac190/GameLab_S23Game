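; Squeeze-through passage actor that lets the player move sideways along a spline through a tight gap.
; The construction script adds capsule triggers at both spline ends; overlaps toggle entering and exiting.
; Entering sets the move mode and travel direction, shrinks the player's capsule and clamps camera yaw; exiting restores them.
; UpdateTransform maps an alpha to spline position, keeping the player's height and turning them 90 degrees off the path.
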(event `self.Trigger_01.OnComponentBeginOverlap`
  (params (OverlappedComponent :type "PrimitiveComponent Object Reference") (OtherActor :type "Actor Object Reference") (OtherComp :type "PrimitiveComponent Object Reference") (OtherBodyIndex :type Integer) (bFromSweep :type Boolean) (SweepResult :type "HitResult Structure (by ref)"))
  (bind _asbp_player (cast `/Game/Entities/Player/BP_Player` OtherActor))
  (set `self.Player` _asbp_player)
  (set `self.CurrentTrigger` (`self.Trigger_01`))
  (if (`self.IsSqueezing`) :!label _label
    (`self.Exit`)
    (else
      (`self.Enter` (`self.CurrentTrigger`)))))

(event `self.Trigger_02.OnComponentBeginOverlap`
  (params (OverlappedComponent :type "PrimitiveComponent Object Reference") (OtherActor :type "Actor Object Reference") (OtherComp :type "PrimitiveComponent Object Reference") (OtherBodyIndex :type Integer) (bFromSweep :type Boolean) (SweepResult :type "HitResult Structure (by ref)"))
  (bind _asbp_player (cast `/Game/Entities/Player/BP_Player` OtherActor))
  (set `self.Player` _asbp_player)
  (set `self.CurrentTrigger` (`self.Trigger_02`))
  (goto _label))

(fn `CreateTrigger`
  (params (Index :type Integer) (Radius :type "Float (double-precision)"))
  (returns (Collider :type "CapsuleComponent Object Reference"))
  (bind _spline (`self.Spline`))
  (bind _returnvalue (`AddComponent|NODE_AddCapsuleComponent-1`))
  (`CapsuleComponent.SetCapsuleSize` _returnvalue Radius 200.0 true)
  (`SceneComponent.K2_SetWorldLocationAndRotation` _returnvalue (+ (`SplineComponent.GetLocationAtSplinePoint` _spline Index "World") (0.0 0.0 130.0)) (`SplineComponent.GetRotationAtSplinePoint` _spline Index "World") false true)
  (return _returnvalue))

(fn `Enter`
  (params (Collider :type "CapsuleComponent Object Reference"))
  (bind _returnvalue (`GameplayStatics.GetPlayerCameraManager` 0))
  (bind (_returnvalue_x _returnvalue_y) (`KismetMathLibrary.BreakVector` (`SceneComponent.K2_GetComponentLocation` (`self.CurrentTrigger`))))
  (bind _viewyawmax (`PlayerCameraManager.ViewYawMax` _returnvalue))
  (bind _viewyawmin (`PlayerCameraManager.ViewYawMin` _returnvalue))
  (bind _capsulecomponent (`Character.CapsuleComponent` (`self.Player`)))
  (bind _success (`/Game/Systems/Player/AC_Movement.SetMoveMode` (`/Game/Entities/Player/BP_Player.AC_Movement` (`self.Player`)) "NewEnumerator3"))
  (if _success
    (set `/Game/Entities/Player/BP_Player.SqueezeInstance` self (`self.Player`))
    ;[1 1 1] Calculate Direction
    (bind _output_get (set `self.IsForwards` (== (`local.Collider`) (`self.Trigger_01`))))
    (`/Game/Entities/Player/BP_Player.SetSqueezeDirection` (`self.Player`) _output_get)
    (set `self.IsSqueezing` true)
    (set `self.Capsule_Size_Original` (`CapsuleComponent.CapsuleRadius` _capsulecomponent))
    (set `self.Clamp_Presqueeze` (`KismetMathLibrary.MakeVector2D` _viewyawmin _viewyawmax)) ; Set the original clamp
    (`CapsuleComponent.SetCapsuleRadius` _capsulecomponent (`self.Capsule_Size_Small`) false)
    (`/Game/Entities/Player/BP_Player.Lerp Transiton And Clamp` (`self.Player`) (`self.AngleClamp`) (`KismetMathLibrary.MakeVector2D` _viewyawmin _viewyawmax) (`KismetMathLibrary.Conv_Vector2DToVector` (`KismetMathLibrary.MakeVector2D` _returnvalue_x _returnvalue_y)))))

(fn `Exit`
  (bind _player (`self.Player`))
  (`/Game/Systems/Player/AC_Movement.SetMoveMode` (`/Game/Entities/Player/BP_Player.AC_Movement` _player) "NewEnumerator0")
  (set `self.IsSqueezing` false)
  (set `self.CurrentTrigger` null)
  (set `/Game/Entities/Player/BP_Player.SqueezeInstance` null _player)
  (`CapsuleComponent.SetCapsuleRadius` (`Character.CapsuleComponent` (`self.Player`)) (`self.Capsule_Size_Original`) false)
  (`/Game/Entities/Player/BP_Player.Lerp Transiton And Clamp` (`self.Player`) (`self.Clamp_Presqueeze`) (0.0 0.0) (0.0 0.0 0.0))
  (set `/Game/Entities/Player/BP_Player.squeezeCameraDivisor` 1.0 (`self.Player`)))

(fn `Update Transform`
  (params (Alpha :type "Float (double-precision)"))
  (bind _player (`self.Player`))
  (bind _spline (`self.Spline`))
  (bind _returnvalue (`KismetMathLibrary.Lerp` 0.0 (`SplineComponent.GetSplineLength` _spline) Alpha))
  (bind (_returnvalue_roll _returnvalue_pitch _returnvalue_yaw) (`KismetMathLibrary.BreakRotator` (`SplineComponent.GetRotationAtDistanceAlongSpline` _spline _returnvalue "World")))
  (`self.K2_SetActorLocationAndRotation` _player (`KismetMathLibrary.MakeVector` (.x (`SplineComponent.GetLocationAtDistanceAlongSpline` _spline _returnvalue "World")) (.y (`SplineComponent.GetLocationAtDistanceAlongSpline` _spline _returnvalue "World")) (.z (`self.K2_GetActorLocation` _player))) (`KismetMathLibrary.MakeRotator` _returnvalue_roll _returnvalue_pitch (- _returnvalue_yaw 90.0)) false false))

(fn `UserConstructionScript`
  (bind _collider (`self.CreateTrigger` 0 (`self.TriggerRange`)))
  (set `self.Trigger_01` _collider)
  (bind _collider_2 (`self.CreateTrigger` (- (`SplineComponent.GetNumberOfSplinePoints` (`self.Spline`)) 1) (`self.TriggerRange`)))
  (set `self.Trigger_02` _collider_2))