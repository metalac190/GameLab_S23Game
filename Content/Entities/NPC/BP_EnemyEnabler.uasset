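; Trigger actor that shows or hides a pre-placed enemy NPC (logged as "Avacado") when the player crosses its spawn and despawn collision volumes.
; The NPC starts hidden with collision and tick off; SpawnCollision re-enables it, teleports it to a random SpawnLocations entry and plays a spawn sound.
; DespawnCollision and the Destroy event hide it again, with MonsterSpawned guarding against repeats.
; An unused reference graph keeps the older single-toggle spawn logic.
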(event `RemoveNPC`
  (bind _npc (`self.NPC`))
  ;[1 1 1] Monster Go Away
  (set `self.MonsterSpawned` false)
  (`self.SetActorHiddenInGame` _npc true)
  (`self.SetActorEnableCollision` _npc false)
  (`self.SetActorTickEnabled` _npc false)
  (`KismetSystemLibrary.PrintString` "[Spawner] Avacado has been hidden" true true (struct :`R` 1.0 :`G` 0.121569 :`B` 0.184314 :`A` 1.0)))

(event `self.ReceiveBeginPlay`
  (bind _npc (`self.NPC`))
  ;[0.2481 0.4079 1] Initial Hide
  (`self.SetActorHiddenInGame` _npc true)
  (`self.SetActorEnableCollision` _npc false)
  (`self.SetActorTickEnabled` _npc false))

(event `self.SpawnCollision.OnComponentBeginOverlap`
  (params (OverlappedComponent :type "PrimitiveComponent Object Reference") (OtherActor :type "Actor Object Reference") (OtherComp :type "PrimitiveComponent Object Reference") (OtherBodyIndex :type Integer) (bFromSweep :type Boolean) (SweepResult :type "HitResult Structure (by ref)"))
  (bind _npc (`self.NPC`))
  (bind _returnvalue (`self.K2_GetActorLocation` (`self.NPC`)))
  ;[0.6265 1 0.1458] SpawnCollision Logic
  (cast `/Game/Entities/Player/BP_Player` OtherActor)
  (if (`self.MonsterSpawned`)
    (`KismetSystemLibrary.PrintString` "[Spawner] Avacado was already spawned." true true (struct :`R` 0.396755 :`G` 0.637597 :`B` 0.093059 :`A` 1.0))
    (else
      (`KismetSystemLibrary.PrintString` "[Spawner] Spawning Avacado..." true true (struct :`R` 0.396078 :`G` 0.635294 :`B` 0.094118 :`A` 1.0))
      (set `self.MonsterSpawned` true)
      (`self.SetActorHiddenInGame` _npc false)
      (`self.SetActorEnableCollision` _npc true)
      (`self.SetActorTickEnabled` _npc true)
      (`self.K2_SetActorLocation` _npc (`KismetArrayLibrary.Array_Random` (`self.SpawnLocations`)) false false)
      (`GameplayStatics.PlaySoundAtLocation` "/Game/Audio/Gameplay/Cues/sfx_creature_spawn.sfx_creature_spawn" _returnvalue (struct) 1.0 1.0 0.0 null null null null)
      (`KismetSystemLibrary.PrintString` (`KismetStringLibrary.Concat_StrStr` "[Spawner] Spawned Avacado at Location -> " (`KismetStringLibrary.Conv_VectorToString` _returnvalue)) true true (struct :`R` 0.396755 :`G` 0.637597 :`B` 0.093059 :`A` 1.0)))))

(event `Destroy`
  (`self.RemoveNPC`)
  (`self.K2_DestroyActor`))

(event `self.DespawnCollision.OnComponentBeginOverlap`
  (params (OverlappedComponent :type "PrimitiveComponent Object Reference") (OtherActor :type "Actor Object Reference") (OtherComp :type "PrimitiveComponent Object Reference") (OtherBodyIndex :type Integer) (bFromSweep :type Boolean) (SweepResult :type "HitResult Structure (by ref)"))
  ;[1 0.125 0.125] DespawnCollision Logic
  (cast `/Game/Entities/Player/BP_Player` OtherActor)
  (if (`self.MonsterSpawned`)
    (`KismetSystemLibrary.PrintString` "[Spawner] Despawning Avacado" true true (struct))
    (`self.RemoveNPC`)
    (else
      (`KismetSystemLibrary.PrintString` "[Spawner] Avacado has already been despawned" true true (struct :`R` 1.0 :`G` 0.121569 :`B` 0.184314 :`A` 1.0)))))

(fn `UserConstructionScript`)