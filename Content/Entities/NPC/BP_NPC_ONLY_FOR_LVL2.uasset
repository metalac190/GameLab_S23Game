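; Level 2 variant of the NPC creature that watches for the player and kills them when they get too close.
; AI_NPC sight events toggle PlayerVisible and play a spotting sound, re-armed after a short delay out of sight.
; Tick optionally aims RotateToPlayer at the visible player and triggers a distance-based kill, gated until the lose menu's reload event.
; Overlapping the Lvl2_SphereOfDeath kills the player directly.
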(event `self.ReceiveBeginPlay`
  (`|ExecutionSequence`
    (:`then_1`
      (bind _asbp_player (cast `/Game/Entities/Player/BP_Player` (`GameplayStatics.GetPlayerPawn` 0)))
      (set `self.Player` _asbp_player))
    (:`then_2`
      (bind _asai_npc (cast `/Game/Systems/NPC/AI_NPC` (`AIBlueprintHelperLibrary.GetAIController` self)))
      (add `/Game/Systems/NPC/AI_NPC.OnPlayerSeen` _asai_npc (delegate `OnPlayerSeen`))
      (add `/Game/Systems/NPC/AI_NPC.OnPlayerLost` _asai_npc (delegate `OnPlayerLost`)))
    (:`then_3`
      (add `/Game/UI/Widgets/WBP_LoseMenu.ReloadGame` (`/Game/Entities/Player/BP_Player.LoseMenuWidget` (`self.Player`)) (delegate `CanKillPlayer`)))))

(event `OnPlayerLost`
  (set `self.PlayerVisible` false)
  (`KismetSystemLibrary.Delay` 2.0) ; arbitrary delay to wait on reseting the spotting sound
  (if (not (`self.PlayerVisible`))
    (goto _label :!via `Reset`)))

(event `OnPlayerSeen`
  (set `self.PlayerVisible` true)
  (`/Engine/EditorBlueprintResources/StandardMacros.DoOnce` false :!label _label
    (:`Completed`
      (`GameplayStatics.PlaySound2D` "/Game/Audio/Gameplay/Cues/sfx_creature_seePlayer.sfx_creature_seePlayer" 1.0 1.0 0.0 null null))))

(event `CanKillPlayer`
  (goto _label_2 :!via `Reset`))

(event `self.ReceiveTick`
  (params (DeltaSeconds :type "Float (single-precision)"))
  (bind _rotatetoplayer (`self.RotateToPlayer`))
  (bind _returnvalue (`SceneComponent.K2_GetComponentLocation` (`self.RotateToPlayer`)))
  (bind _returnvalue_2 (`SceneComponent.K2_GetComponentLocation` (`Actor.RootComponent` (`self.Player`))))
  (if (`self.RotateTentacles`)
    (if (`self.PlayerVisible`)
      (`SceneComponent.K2_SetWorldRotation` _rotatetoplayer (`KismetMathLibrary.FindLookAtRotation` _returnvalue _returnvalue_2) false false)
      (else
        (`SceneComponent.K2_SetRelativeRotation` :`self` _rotatetoplayer))))
  (if (< (`KismetMathLibrary.Vector_Distance` _returnvalue _returnvalue_2) (`self.DistToKill`))
    (`/Engine/EditorBlueprintResources/StandardMacros.DoOnce` false :!label _label_2 ; only calls KillPlayer once until the level is reloaded
      (:`Completed`
        (`KismetSystemLibrary.PrintString` "PLAYER IS DEAD")
        (`/Game/Entities/Player/BP_Player.KillPlayer` (`self.Player`))))))

(event `self.Lvl2_SphereOfDeath.OnComponentBeginOverlap`
  (params (OverlappedComponent :type "PrimitiveComponent Object Reference") (OtherActor :type "Actor Object Reference") (OtherComp :type "PrimitiveComponent Object Reference") (OtherBodyIndex :type Integer) (bFromSweep :type Boolean) (SweepResult :type "HitResult Structure (by ref)"))
  (bind _asbp_player (cast `/Game/Entities/Player/BP_Player` OtherActor))
  (`/Game/Entities/Player/BP_Player.KillPlayer` _asbp_player))

(fn `UserConstructionScript`)