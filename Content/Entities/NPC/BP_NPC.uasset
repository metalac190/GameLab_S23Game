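; BP_NPC is a creature that spots the player and kills them within a set range.
; AI_NPC sight events toggle visibility, triggering a sound and force feedback, with a delayed reset to avoid repeated stingers.
; Tick optionally turns the tentacles toward the visible player and checks kill distance.
; A DoOnce limits the kill to one call, re-armed by the lose menu's reload event.
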(event `self.ReceiveBeginPlay`
  (bind _forcefeedback (`self.ForceFeedback`))
  (bind (_attenuationoverrides_distancealgorithm _attenuationoverrides_attenuationshape _attenuationoverrides_falloffmode _attenuationoverrides_dbattenuationatmax _attenuationoverrides_attenuationshapeextents _attenuationoverrides_coneoffset _attenuationoverrides_falloffdistance) (break `ForceFeedbackAttenuationSettings` (`ForceFeedbackComponent.AttenuationOverrides` _forcefeedback)))
  (`KismetSystemLibrary.DrawDebugSphere` (`SceneComponent.K2_GetComponentLocation` _forcefeedback) _attenuationoverrides_falloffdistance)
  (`|ExecutionSequence`
    (:`then_0`
      (bind _asbp_player (cast `/Game/Entities/Player/BP_Player` (`GameplayStatics.GetPlayerPawn` 0)))
      (set `self.Player` _asbp_player))
    (:`then_1`
      (bind _asai_npc (cast `/Game/Systems/NPC/AI_NPC` (`AIBlueprintHelperLibrary.GetAIController` self)))
      (add `/Game/Systems/NPC/AI_NPC.OnPlayerSeen` _asai_npc (delegate `OnPlayerSeen`))
      (add `/Game/Systems/NPC/AI_NPC.OnPlayerLost` _asai_npc (delegate `OnPlayerLost`)))
    (:`then_2`
      (add `/Game/UI/Widgets/WBP_LoseMenu.ReloadGame` (`/Game/Entities/Player/BP_Player.LoseMenuWidget` (`self.Player`)) (delegate `CanKillPlayer`)))))

(event `OnPlayerSeen`
  (set `self.PlayerVisible` true)
  (`/Engine/EditorBlueprintResources/StandardMacros.DoOnce` false :!label _label
    (:`Completed`
      (`GameplayStatics.PlaySound2D` "/Game/Audio/Gameplay/Cues/sfx_creature_seePlayer.sfx_creature_seePlayer" 1.0 1.0 0.0 null null)
      (`ForceFeedbackComponent.Play` (`self.ForceFeedback`) 0.0))))

(event `OnPlayerLost`
  (set `self.PlayerVisible` false)
  (`KismetSystemLibrary.Delay` 2.0) ; arbitrary delay to wait on reseting the spotting sound
  (if (not (`self.PlayerVisible`))
    (goto _label :!via `Reset`)))

(event `CanKillPlayer`
  (goto _label_2 :!via `Reset`))

(event `self.ReceiveTick`
  (params (DeltaSeconds :type "Float (single-precision)"))
  (bind _returnvalue (`SceneComponent.K2_GetComponentLocation` (`self.RotateToPlayer`)))
  (bind _returnvalue_2 (`SceneComponent.K2_GetComponentLocation` (`Actor.RootComponent` (`self.Player`))))
  (if (`self.RotateTentacles`)
    (if (`self.PlayerVisible`)
      (`SceneComponent.K2_SetWorldRotation` (`self.RotateToPlayer`) (`KismetMathLibrary.FindLookAtRotation` _returnvalue _returnvalue_2) false false)
      (else
        (`SceneComponent.K2_SetRelativeRotation` :`self` (`self.RotateToPlayer`)))))
  (if (< (`KismetMathLibrary.Vector_Distance` _returnvalue _returnvalue_2) (`self.DistToKill`))
    (`/Engine/EditorBlueprintResources/StandardMacros.DoOnce` false :!label _label_2 ; only calls KillPlayer once until the level is reloaded
      (:`Completed`
        (`KismetSystemLibrary.PrintString` "PLAYER IS DEAD")
        (`/Game/Entities/Player/BP_Player.KillPlayer` (`self.Player`))
        (`ForceFeedbackComponent.Stop` (`self.ForceFeedback`))))))

(fn `UserConstructionScript`)