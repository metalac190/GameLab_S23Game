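; BP_NPC_DummyController drives a scripted monster pass through an area, tied to a HideSequence.
; The monster starts disabled (hidden, no collision or tick) and spawns on SpawnMonster, automatically after a delay if MoveOnStart is set.
; Spawning teleports the existing monster to Start, then chains AI moves to the HideSequence's travel point and End.
; Failed moves continue like successes, so the monster always gets disabled and CallMonsterClearedArea fires.
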(event `self.ReceiveBeginPlay`
  (`self.EnableMonster` false)
  (if (`self.MoveOnStart`)
    (`KismetSystemLibrary.Delay` 5.0)
    (`self.SpawnMonster`)))

(event `SpawnMonster`
  (bind _end_location (`KismetMathLibrary.BreakTransform` (`self.End`)))
  (`self.EnableMonster` true)
  (`SceneComponent.K2_SetWorldTransform` (`Actor.RootComponent` (`self.Monster`)) (`self.Start`) false true)
  (bind _location (`/Game/Entities/Gameplay/HidingSequence/BP_HideSequence.GetMonsterTravelTo` (`self.HideSequence`)))
  (`|AIMoveTo` (`self.Monster`) _location null 50.0
    (:`OnSuccess`
      _)
    (:`OnFail`
      _))
  (`|AIMoveTo` (`self.Monster`) _end_location null 50.0
    (:`OnSuccess`
      _)
    (:`OnFail`
      _))
  (`self.EnableMonster` false)
  (`self.MonsterClearedArea`))

(fn `EnableMonster`
  (params (Enabled :type Boolean))
  (bind _monster (`self.Monster`))
  (`self.SetActorHiddenInGame` _monster (not Enabled))
  (`self.SetActorEnableCollision` _monster Enabled)
  (`self.SetActorTickEnabled` _monster Enabled))

(fn `UserConstructionScript`)