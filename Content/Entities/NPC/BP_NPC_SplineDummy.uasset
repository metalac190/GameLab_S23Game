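; BP_NPC_SplineDummy is a monster NPC that travels a spline path from its HideSequence, apparently as part of a player hiding sequence.
; Starting the path shows the monster, and Tick moves it by distance along the spline at a set Speed.
; Reaching the end hides it and fires CompletedMonsterSpline, while FailedHide stops movement and re-enables its AI_NPC controller.
; The proximity kill check on the player is unconnected and never runs.
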(event `self.ReceiveBeginPlay`
  (bind _asbp_player (cast `/Game/Entities/Player/BP_Player` (`GameplayStatics.GetPlayerPawn` 0)))
  (set `self.Player` _asbp_player)
  (bind _asai_npc (cast `/Game/Systems/NPC/AI_NPC` (`AIBlueprintHelperLibrary.GetAIController` self)))
  (`/Game/Systems/NPC/AI_NPC.PlayerHidden` _asai_npc)
  (`self.SetMonsterEnabled` false)
  (if (`self.AutoActivate`)
    (`self.StartMonsterFollowSplinePath`)))

(event `self.ReceiveTick`
  (params (DeltaSeconds :type "Float (single-precision)"))
  (bind _spline_path (`self.Spline Path`))
  (if (`self.MoveOnSpline`)
    (bind _output_get (set `self.SplineDelta` (+ (`self.SplineDelta`) (* DeltaSeconds (`self.Speed`)))))
    (if (> _output_get (`SplineComponent.GetSplineLength` _spline_path))
      (`self.SetMonsterEnabled` false)
      (`KismetSystemLibrary.PrintString` "Monster Completed Spline. Notify Level Blueprint")
      (`self.CompletedMonsterSpline`)
      (else
        (bind (_returnvalue _returnvalue2) (`self.GetSplineLocRot` _spline_path _output_get))
        (`SceneComponent.K2_SetWorldLocationAndRotation` (`self.CapsuleComponent`) (+ _returnvalue (0.0 0.0 90.0)) _returnvalue2 false false)))))

(event `StartMonsterFollowSplinePath`
  (bind _splinepath (`/Game/Entities/Gameplay/HidingSequence/BP_HideSequence.GetMonsterSplinePath` (`self.HideSequence`)))
  (`/Engine/EditorBlueprintResources/StandardMacros.IsValid` _splinepath
    (:`Is Valid`
      (set `self.Spline Path` _splinepath)
      (set `self.SplineDelta` 0.0)
      (`self.SetMonsterEnabled` true))
    (:`Is Not Valid`
      (`KismetSystemLibrary.PrintString` "No Valid Spline for Monster"))))

(event `FailedHide`
  (set `self.MoveOnSpline` false)
  (bind _asai_npc (cast `/Game/Systems/NPC/AI_NPC` (`AIBlueprintHelperLibrary.GetAIController` self)))
  (set `/Game/Systems/NPC/AI_NPC.AIDisabled` false _asai_npc)
  (`KismetSystemLibrary.PrintString` "AI is Now Enabled"))

(fn `GetSplineLocRot`
  (params (Spline :type "SplineComponent Object Reference") (Distance :type "Float (double-precision)"))
  (returns (ReturnValue :type "Vector Structure") (ReturnValue2 :type "Rotator Structure"))
  (return (`SplineComponent.GetLocationAtDistanceAlongSpline` Spline Distance "World") (`SplineComponent.GetRotationAtDistanceAlongSpline` Spline Distance "World")))

(fn `SetMonsterEnabled`
  (params (Enabled :type Boolean))
  (bind _output_get (set `self.MoveOnSpline` Enabled))
  (`SceneComponent.SetVisibility` (`self.CapsuleComponent`) _output_get true))

(fn `UserConstructionScript`)