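; BP_NPC_Dummy is a placeholder NPC that kills the player on proximity.
; BeginPlay caches the first player pawn as a BP_Player.
; Every Tick compares the distance between its capsule and the player's root against DistToKill, then prints a debug message and calls KillPlayer while within range.
; The graph contains no movement or AI logic, and the kill has no once-only guard.
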(event `self.ReceiveBeginPlay`
  (bind _asbp_player (cast `/Game/Entities/Player/BP_Player` (`GameplayStatics.GetPlayerPawn` 0)))
  (set `self.Player` _asbp_player))

(event `self.ReceiveTick`
  (params (DeltaSeconds :type "Float (single-precision)"))
  (if (< (`KismetMathLibrary.Vector_Distance` (`SceneComponent.K2_GetComponentLocation` (`self.CapsuleComponent`)) (`SceneComponent.K2_GetComponentLocation` (`Actor.RootComponent` (`self.Player`)))) (`self.DistToKill`))
    (`KismetSystemLibrary.PrintString` "PLAYER IS DEAD")
    (`/Game/Entities/Player/BP_Player.KillPlayer` (`self.Player`))))

(fn `UserConstructionScript`)